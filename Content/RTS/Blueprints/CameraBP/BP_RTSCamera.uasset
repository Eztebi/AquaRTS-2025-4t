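; RTS camera pawn that pans by input or screen-edge cursor, zooms via spring arm length, and handles unit selection and orders.
; Left-click cursor traces fill unit or building selection arrays and send select/deselect messages to units.
; Right-click traces branch on hit class, ordering Aldeano_BP villagers to act on resources and other units on characters or buildings, otherwise moving them.
; Several click helper functions duplicate inline logic and go uncalled here.
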(event `EnhancedInput|/Game/RTS/Inputs/SelectionInput/IA_Selection`
  (params (ActionValue :type Boolean) (ElapsedSeconds :type "Float (double-precision)") (TriggeredSeconds :type "Float (double-precision)") (InputAction :type "InputAction Object Reference" :default "/Game/RTS/Inputs/SelectionInput/IA_Selection.IA_Selection"))
  (bind (_worldlocation _worlddirection) (`PlayerController.DeprojectMousePositionToWorld` (`GameplayStatics.GetPlayerController` 0)))
  ; LeftClick
  (:`Triggered`
    (bind _outhit (`KismetSystemLibrary.LineTraceSingle` _worldlocation (+ _worldlocation (* _worlddirection 10000.0)) "TraceTypeQuery1"))
    (`self.LeftClickedActor` _outhit)))

(event `EnhancedInput|/Game/RTS/Inputs/CameraInput/IA_CameraMove`
  (params (ActionValue :type "Vector2D Structure") (ElapsedSeconds :type "Float (double-precision)") (TriggeredSeconds :type "Float (double-precision)") (InputAction :type "InputAction Object Reference" :default "/Game/RTS/Inputs/CameraInput/IA_CameraMove.IA_CameraMove"))
  (bind (_x _y) (`KismetMathLibrary.BreakVector2D` ActionValue))
  ; Camera
  ;; Camera Move
  (:`Triggered`
    (`self.MoveForward` _x)
    (`self.MoveRight` _y)))

(event `EnhancedInput|/Game/RTS/Inputs/CameraInput/IA_Zoom`
  (params (ActionValue :type "Float (double-precision)") (ElapsedSeconds :type "Float (double-precision)") (TriggeredSeconds :type "Float (double-precision)") (InputAction :type "InputAction Object Reference" :default "/Game/RTS/Inputs/CameraInput/IA_Zoom.IA_Zoom"))
  (bind _springarm (`self.SpringArm`))
  ; Camera
  ;; Camera Zoom
  (:`Triggered`
    (set `SpringArmComponent.TargetArmLength` (`KismetMathLibrary.FClamp` (+ (`SpringArmComponent.TargetArmLength` _springarm) (* ActionValue (`self.zoomSpeed`))) 20.0 1000.0) _springarm)))

(event `EnhancedInput|/Game/RTS/Inputs/SelectionInput/IA_Action`
  (params (ActionValue :type Boolean) (ElapsedSeconds :type "Float (double-precision)") (TriggeredSeconds :type "Float (double-precision)") (InputAction :type "InputAction Object Reference" :default "/Game/RTS/Inputs/SelectionInput/IA_Action.IA_Action"))
  (bind (_worldlocation _worlddirection) (`PlayerController.DeprojectMousePositionToWorld` (`GameplayStatics.GetPlayerController` 0)))
  ; Right Click
  (:`Triggered`
    (bind _outhit (`KismetSystemLibrary.LineTraceSingle` _worldlocation (+ _worldlocation (* _worlddirection 10000.0)) "TraceTypeQuery1"))
    (if (`KismetArrayLibrary.Array_IsNotEmpty` (`self.ActorArray`))
      (bind (_bblockinghit _binitialoverlap _time _distance _location _impactpoint _normal _impactnormal _physmat _hitactor) (`GameplayStatics.BreakHitResult` _outhit))
      ;; RightClickedCharacter
      (if (`GameplayStatics.ObjectIsA` _hitactor "/Script/AquaRTS.CharacterRTS")
        (for _array_element (`self.ActorArray`)
          (if (`GameplayStatics.ObjectIsA` _array_element "/Game/RTS/Blueprints/CharactersBP/Aldeano_BP.Aldeano_BP_C")
            (bind _ascharacter_rts (cast `CharacterRTS` _array_element))
            (`CharacterRTS.Move` _ascharacter_rts (`self.K2_GetActorLocation`))
            (else
              (bind _ascharacter_rts_2 (cast `CharacterRTS` _array_element))
              (`CharacterRTS.Action` _ascharacter_rts_2 _hitactor))))
        (else
          ;; RightClickedBuilding
          (if (`GameplayStatics.ObjectIsA` _hitactor "/Script/AquaRTS.Building")
            (for _array_element_2 (`self.ActorArray`)
              (if (`GameplayStatics.ObjectIsA` _array_element_2 "/Game/RTS/Blueprints/CharactersBP/Aldeano_BP.Aldeano_BP_C")
                (bind _ascharacter_rts_3 (cast `CharacterRTS` _array_element_2))
                (`CharacterRTS.Move` _ascharacter_rts_3 (`self.K2_GetActorLocation` _hitactor))
                (else
                  (bind _ascharacter_rts_4 (cast `CharacterRTS` _array_element_2))
                  (`CharacterRTS.Action` _ascharacter_rts_4 _hitactor))))
            (else
              ;; RightClickedResource
              (if (`GameplayStatics.ObjectIsA` _hitactor "/Script/AquaRTS.Resource")
                (for _array_element_3 (`self.ActorArray`)
                  (if (`GameplayStatics.ObjectIsA` _array_element_3 "/Game/RTS/Blueprints/CharactersBP/Aldeano_BP.Aldeano_BP_C")
                    (bind _ascharacter_rts_5 (cast `CharacterRTS` _array_element_3))
                    (`CharacterRTS.Action` _ascharacter_rts_5 _hitactor)
                    (else
                      (bind _ascharacter_rts_6 (cast `CharacterRTS` _array_element_3))
                      (`CharacterRTS.Move` _ascharacter_rts_6 (`self.K2_GetActorLocation` _hitactor)))))
                (else
                  ;; RightClickedPosition
                  (for _array_element_4 (`self.ActorArray`)
                    (bind _ascharacter_rts_7 (cast `CharacterRTS` _array_element_4))
                    (`CharacterRTS.Move` _ascharacter_rts_7 _location))))))))
      (else
        (`KismetSystemLibrary.PrintText` "Nothing Selected")))))

(event `self.ReceiveBeginPlay`
  (bind _returnvalue (`GameplayStatics.GetPlayerController` 0))
  ; Camera
  ;; Show cursor
  (`|ExecutionSequence`
    (:`then_0`
      (`WidgetBlueprintLibrary.SetInputMode_GameAndUIEx` _returnvalue null "LockAlways" false)
      (set `PlayerController.bShowMouseCursor` true _returnvalue))))

(event `InputAxisKey|MouseY`
  (params (AxisValue :type "Float (single-precision)"))
  (bind (_returnvalue_x _returnvalue_y) (`KismetMathLibrary.BreakVector2D` (`WidgetLayoutLibrary.GetViewportSize`)))
  (bind _returnvalue (/ (`PlayerController.GetMousePosition` (`GameplayStatics.GetPlayerController` 0)) _returnvalue_x))
  ; Camera
  ;; Cursor move
  (if (> _returnvalue 0.98)
    (`self.MoveRight` 1.0)
    (elif (< _returnvalue 0.02)
      (`self.MoveRight` -1.0))))

(event `InputAxisKey|MouseX`
  (params (AxisValue :type "Float (single-precision)"))
  (bind (_returnvalue_x _returnvalue_y) (`KismetMathLibrary.BreakVector2D` (`WidgetLayoutLibrary.GetViewportSize`)))
  (bind _returnvalue (/ (`.LocationY` (`PlayerController.GetMousePosition` (`GameplayStatics.GetPlayerController` 0))) _returnvalue_y))
  ; Camera
  ;; Cursor move
  (if (> _returnvalue 0.98)
    (`self.MoveForward` -1.0)
    (elif (< _returnvalue 0.02)
      (`self.MoveForward` 1.0))))

(fn `LeftClickedActor`
  (params (Hit :type "HitResult Structure (by ref)"))
  (bind (_bblockinghit _binitialoverlap _time _distance _location _impactpoint _normal _impactnormal _physmat _hitactor) (`GameplayStatics.BreakHitResult` Hit))
  (bind _actorarray (`self.ActorArray`))
  (bind _actorarray_2 (`self.ActorArray`))
  ; LeftClickedCharacter
  (if (`GameplayStatics.ObjectIsA` _hitactor "/Script/AquaRTS.CharacterRTS")
    (for _array_element (`self.ActorArray`)
      (message `ISelectionTroop.OnDeselected` _array_element))
    (`KismetArrayLibrary.Array_Clear` (`self.ActorArray`))
    (`KismetArrayLibrary.Array_AddUnique` (`self.ActorArray`) _hitactor)
    (`KismetArrayLibrary.Array_Clear` (`self.BuildingArray`))
    (for _array_element_2 (`self.ActorArray`)
      (message `ISelectionTroop.OnSelected` _array_element_2)
      (`KismetSystemLibrary.PrintText` (`KismetTextLibrary.Conv_ObjectToText` _array_element_2)))
    (else
      ; LeftClickedBuilding
      (if (`GameplayStatics.ObjectIsA` _hitactor "/Script/AquaRTS.Building")
        (for _array_element_3 _actorarray_2
          (message `ISelectionTroop.OnDeselected` _array_element_3))
        (`KismetArrayLibrary.Array_Clear` _actorarray_2)
        (`KismetArrayLibrary.Array_AddUnique` (`self.BuildingArray`) _hitactor)
        (else
          ; LeftClickedPosition
          (for _array_element_4 _actorarray
            (message `ISelectionTroop.OnDeselected` _array_element_4))
          (`KismetArrayLibrary.Array_Clear` _actorarray)
          (`KismetArrayLibrary.Array_Clear` (`self.BuildingArray`)))))))

(fn `LeftClickedBuilding`
  (params (NewItem :type "Actor Object Reference (by ref)") (Object :type "Object Object Reference"))
  (bind _actorarray (`self.ActorArray`))
  (if (`GameplayStatics.ObjectIsA` Object "/Script/AquaRTS.Building")
    (for _array_element _actorarray
      (message `ISelectionTroop.OnDeselected` _array_element))
    (`KismetArrayLibrary.Array_Clear` _actorarray)
    (`KismetArrayLibrary.Array_AddUnique` (`self.BuildingArray`) NewItem)))

(fn `LeftClickedCharacter`
  (params (Object :type "Object Object Reference") (NewItem :type "Actor Object Reference (by ref)"))
  (if (`GameplayStatics.ObjectIsA` Object "/Script/AquaRTS.CharacterRTS")
    (`KismetArrayLibrary.Array_Clear` (`self.ActorArray`))
    (`KismetArrayLibrary.Array_AddUnique` (`self.ActorArray`) NewItem)
    (`KismetArrayLibrary.Array_Clear` (`self.BuildingArray`))
    (for _array_element (`self.ActorArray`)
      (message `ISelectionTroop.OnSelected` _array_element)
      (`KismetSystemLibrary.PrintText` (`KismetTextLibrary.Conv_ObjectToText` _array_element)))))

(fn `LeftClickedPosition`
  (bind _actorarray (`self.ActorArray`))
  (for _array_element _actorarray
    (message `ISelectionTroop.OnDeselected` _array_element))
  (`KismetArrayLibrary.Array_Clear` _actorarray)
  (`KismetArrayLibrary.Array_Clear` (`self.BuildingArray`)))

(fn `MoveForward`
  (params (ScaleValue :type "Float (single-precision)"))
  (`self.AddMovementInput` (`self.GetActorForwardVector`) ScaleValue))

(fn `MoveRight`
  (params (ScaleValue :type "Float (single-precision)"))
  (`self.AddMovementInput` (`self.GetActorRightVector`) ScaleValue))

(fn `RightClickedBuilding`
  (params (self2 :type "Actor Object Reference") (tempTarget :type "Actor Object Reference") (object :type "Object Object Reference"))
  (if (`GameplayStatics.ObjectIsA` object "/Script/AquaRTS.Building")
    (for _array_element (`self.ActorArray`)
      (if (`GameplayStatics.ObjectIsA` _array_element "/Game/RTS/Blueprints/CharactersBP/Aldeano_BP.Aldeano_BP_C")
        (bind _ascharacter_rts (cast `CharacterRTS` _array_element))
        (`CharacterRTS.Move` _ascharacter_rts (`self.K2_GetActorLocation` self2))
        (else
          (bind _ascharacter_rts_2 (cast `CharacterRTS` _array_element))
          (`CharacterRTS.Action` _ascharacter_rts_2 tempTarget))))))

(fn `RightClickedCharacter`
  (params (tempTarget :type "Actor Object Reference") (self2 :type "Actor Object Reference") (Object :type "Object Object Reference"))
  (if (`GameplayStatics.ObjectIsA` Object "/Script/AquaRTS.CharacterRTS")
    (for _array_element (`self.ActorArray`)
      (if (`GameplayStatics.ObjectIsA` _array_element "/Game/RTS/Blueprints/CharactersBP/Aldeano_BP.Aldeano_BP_C")
        (bind _ascharacter_rts (cast `CharacterRTS` _array_element))
        (`CharacterRTS.Move` _ascharacter_rts (`self.K2_GetActorLocation` self2))
        (else
          (bind _ascharacter_rts_2 (cast `CharacterRTS` _array_element))
          (`CharacterRTS.Action` _ascharacter_rts_2 tempTarget))))))

(fn `RightClickedPosition`
  (params (location :type "Vector Structure"))
  (for _array_element (`self.ActorArray`)
    (bind _ascharacter_rts (cast `CharacterRTS` _array_element))
    (`CharacterRTS.Move` _ascharacter_rts location)))

(fn `RightClickedResource`
  (params (tempTarget :type "Actor Object Reference") (self2 :type "Actor Object Reference") (object :type "Object Object Reference"))
  (if (`GameplayStatics.ObjectIsA` object "/Script/AquaRTS.Resource")
    (for _array_element (`self.ActorArray`)
      (if (`GameplayStatics.ObjectIsA` _array_element "/Game/RTS/Blueprints/CharactersBP/Aldeano_BP.Aldeano_BP_C")
        (bind _ascharacter_rts (cast `CharacterRTS` _array_element))
        (`CharacterRTS.Action` _ascharacter_rts tempTarget)
        (else
          (bind _ascharacter_rts_2 (cast `CharacterRTS` _array_element))
          (`CharacterRTS.Move` _ascharacter_rts_2 (`self.K2_GetActorLocation` self2)))))))

(fn `UserConstructionScript`)