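; BP_MainCoral is an RTS building Blueprint for the main coral, which flashes a tint color when clicked.
; On BeginPlay, its BPRuntimeMaterial component applies a runtime material to the coral mesh.
; Clicking the Box component runs a short looping yoyo tween that blends the material's tint parameter from its current value toward TintColor.
; A Fresnel mask setter is present but never runs.
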(event `self.ReceiveBeginPlay`
  (`/Game/RTS/Blueprints/BP_RuntimeMaterial.ApplyRuntimeMaterial` (`self.BP_RuntimeMaterial`) (`|MakeArray` (`self.SM_MainCoral`) :!type "MeshComponent Object Reference")))

(event `self.Box.OnClicked`
  (params (TouchedComponent :type "PrimitiveComponent Object Reference") (ButtonPressed :type "Key Structure"))
  (bind _runtimematerial (`/Game/RTS/Blueprints/BP_RuntimeMaterial.runtimeMaterial` (`self.BP_RuntimeMaterial`)))
  (bind _returnvalue (`MaterialInstanceDynamic.K2_GetVectorParameterValue` _runtimematerial (`self.tintParameter`)))
  (bind (_asynctaskproxy _value) (`FCTweenBPActionVector.TweenVector` (`KismetMathLibrary.Conv_LinearColorToVector` _returnvalue) (`KismetMathLibrary.Conv_LinearColorToVector` (`KismetMathLibrary.Conv_ColorToLinearColor` (`self.TintColor`))) 0.25 "Linear" 0.0 0.0 0.0 4 0.0 true)
    (:`ApplyEasing`
      (`MaterialInstanceDynamic.SetVectorParameterValue` _runtimematerial (`self.tintParameter`) (`KismetMathLibrary.Conv_VectorToLinearColor` _value)))))

(fn `UserConstructionScript`)