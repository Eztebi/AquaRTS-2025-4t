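; Capturable food coral zone for the RTS that flags units inside as safe, ignores sharks and tints its overhead UI by owning side.
; An opposing unit's entry starts a dice battle, gathering both sides after a delay and animating MyGameManager rolls on the HUD with timers.
; Fight adjusts both totals by unit-class matchups with tweened point popups.
; Ties reroll; otherwise Winner kills the losing units and sets ownership.
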(event `self.ReceiveBeginPlay`
  (`WidgetComponent.SetTintColorAndOpacity` (`self.OverheadUI`) (struct :`A` 0.501)))

(event `self.Sphere.OnComponentBeginOverlap`
  (params (OverlappedComponent :type "PrimitiveComponent Object Reference") (OtherActor :type "Actor Object Reference") (OtherComp :type "PrimitiveComponent Object Reference") (OtherBodyIndex :type Integer) (bFromSweep :type Boolean) (SweepResult :type "HitResult Structure (by ref)"))
  (if (not (`GameplayStatics.ObjectIsA` OtherActor "/Game/RTS/Blueprints/CharactersBP/Shark_BP.Shark_BP_C"))
    (`self.CharacterEnter` OtherActor)
    (bind _check (`self.CheckForFight` OtherActor))
    (if _check
      (if (not (`self.isCheckingForAllCharacters`))
        (`self.CheckAllCharactersInArea`)))))

(event `self.Sphere.OnComponentEndOverlap`
  (params (OverlappedComponent :type "PrimitiveComponent Object Reference") (OtherActor :type "Actor Object Reference") (OtherComp :type "PrimitiveComponent Object Reference") (OtherBodyIndex :type Integer))
  (if (not (`GameplayStatics.ObjectIsA` OtherActor "/Game/RTS/Blueprints/CharactersBP/Shark_BP.Shark_BP_C"))
    (`self.CharacterExit` OtherActor)))

(event `CheckAllCharactersInArea`
  (bind _sphere (`self.Sphere`))
  (set `self.isCheckingForAllCharacters` true)
  (`KismetSystemLibrary.Delay` 2.0)
  (`KismetArrayLibrary.Array_Clear` (`self.PlayerCharacters`))
  (`KismetArrayLibrary.Array_Clear` (`self.EnemyCharacters`))
  (for _array_element (`PrimitiveComponent.GetOverlappingActors` _sphere "/Script/AquaRTS.CharacterRTS")
    (bind _ascharacter_rts (cast `CharacterRTS` _array_element))
    (`KismetArrayLibrary.Array_Add` (`self.PlayerCharacters`) _ascharacter_rts))
  (for _array_element_2 (`PrimitiveComponent.GetOverlappingActors` _sphere "/Script/AquaRTS.EnemyCharacterRTS")
    (bind _asenemy_character_rts (cast `EnemyCharacterRTS` _array_element_2))
    (`KismetArrayLibrary.Array_Add` (`self.EnemyCharacters`) _asenemy_character_rts))
  (`self.ShowDice` :!label _label)
  (`GameplayStatics.PlaySound2D` "/Game/RTS/Audio/FX/Battle/SC_ThrowDice_Cue.SC_ThrowDice_Cue" 1.0 1.0 0.0 null null)
  (set `self.CurrentTimeDiceEnemy` 0.0)
  (set `self.CurrentTimeDicePlayer` 0.0)
  (bind _returnvalue (`KismetSystemLibrary.K2_SetTimerDelegate` (delegate `DiceEnemyAnimation`) 0.2 (< (`self.CurrentTimeDiceEnemy`) (`self.FinalTimeDice`))))
  (set `self.EnemyTimerHandle` _returnvalue))

(event `DicePlayerAnimation`
  (if (< (`self.CurrentTimeDicePlayer`) (`self.FinalTimeDice`))
    (set `self.CurrentTimeDicePlayer` (+ (`self.CurrentTimeDicePlayer`) 0.2))
    (bind _gameplayhud (`self.GetUserHUDReference`))
    (set `TextBlock.Text` (`KismetTextLibrary.Conv_IntToText` (`KismetMathLibrary.RandomIntegerInRange` 1 6)) (`/Game/RTS/Blueprints/WidgetBP/HUD_WBP.PlayerDice_txt` _gameplayhud))
    (else
      (`KismetSystemLibrary.K2_ClearAndInvalidateTimerHandle` (`self.PlayerTimerHandle`))
      (bind _gameplayhud_2 (`self.GetUserHUDReference`))
      (bind _manager (`self.GetManagerReference`))
      (bind _asmy_game_manager (cast `/Game/RTS/Blueprints/MyGameManager` _manager))
      (bind _playerdicepoints (`/Game/RTS/Blueprints/MyGameManager.PlayerDicePoints` _asmy_game_manager))
      (set `TextBlock.Text` (`KismetTextLibrary.Conv_IntToText` _playerdicepoints) (`/Game/RTS/Blueprints/WidgetBP/HUD_WBP.PlayerDice_txt` _gameplayhud_2))
      (set `self.PlayerPoints` _playerdicepoints)
      (`KismetSystemLibrary.PrintText` "Finished Player Dice" true true (struct :`G` 1.0 :`B` 0.345177 :`A` 1.0))
      (`KismetSystemLibrary.Delay` 2.0)
      (`self.Fight`)
      (if (== (`self.PlayerPoints`) (`self.EnemyPoints`))
        (`KismetSystemLibrary.Delay` 0.5)
        (goto _label)
        (else
          (`KismetSystemLibrary.Delay` 1.0)
          (`self.Winner`)
          (`KismetSystemLibrary.PrintText` "Over")
          (`KismetSystemLibrary.Delay` 2.0)
          (bind _gameplayhud_3 (`self.GetUserHUDReference`))
          (`/Game/RTS/Blueprints/WidgetBP/HUD_WBP.RemoveDicePanel` _gameplayhud_3)
          (set `self.isCheckingForAllCharacters` false))))))

(event `DiceEnemyAnimation`
  (if (< (`self.CurrentTimeDiceEnemy`) (`self.FinalTimeDice`))
    (set `self.CurrentTimeDiceEnemy` (+ (`self.CurrentTimeDiceEnemy`) 0.2))
    (bind _gameplayhud (`self.GetUserHUDReference`))
    (set `TextBlock.Text` (`KismetTextLibrary.Conv_IntToText` (`KismetMathLibrary.RandomIntegerInRange` 1 6)) (`/Game/RTS/Blueprints/WidgetBP/HUD_WBP.EnemyDice_txt` _gameplayhud))
    (else
      (`KismetSystemLibrary.K2_ClearAndInvalidateTimerHandle` (`self.EnemyTimerHandle`))
      (bind _gameplayhud_2 (`self.GetUserHUDReference`))
      (bind _manager (`self.GetManagerReference`))
      (bind _asmy_game_manager (cast `/Game/RTS/Blueprints/MyGameManager` _manager))
      (bind _enemydicepoints (`/Game/RTS/Blueprints/MyGameManager.EnemyDicePoints` _asmy_game_manager))
      (set `TextBlock.Text` (`KismetTextLibrary.Conv_IntToText` _enemydicepoints) (`/Game/RTS/Blueprints/WidgetBP/HUD_WBP.EnemyDice_txt` _gameplayhud_2))
      (set `self.EnemyPoints` _enemydicepoints)
      (`KismetSystemLibrary.PrintText` "Finished Enemy Dice" true true (struct :`R` 1.0 :`B` 0.291467 :`A` 1.0))
      (`KismetSystemLibrary.Delay` 1.0)
      (`GameplayStatics.PlaySound2D` "/Game/RTS/Audio/FX/Battle/SC_ThrowDice_Cue.SC_ThrowDice_Cue" 1.0 1.0 0.0 null null)
      (bind _returnvalue (`KismetSystemLibrary.K2_SetTimerDelegate` (delegate `DicePlayerAnimation`) 0.2 (< (`self.CurrentTimeDicePlayer`) (`self.FinalTimeDice`))))
      (set `self.PlayerTimerHandle` _returnvalue))))

(event `Fight`
  ; Player Points
  (set `self.FightFinished` false)
  (for _array_element (`self.PlayerCharacters`)
    (if (`GameplayStatics.ObjectIsA` _array_element "/Game/RTS/Blueprints/CharactersBP/Player/Recolector_BP.Recolector_BP_C")
      (for _array_element_2 (`self.EnemyCharacters`)
        (if (`GameplayStatics.ObjectIsA` _array_element_2 "/Game/RTS/Blueprints/CharactersBP/Enemy/EnemyRecolector_BP.EnemyRecolector_BP_C")
          (set `self.PointAdded` 1)
          (set `self.PlayerPoints` (+ (`self.PlayerPoints`) (`self.PointAdded`)))
          (`FCTweenBPActionFloat.TweenFloat` 0.0 1.0 1.0 "Linear" :!label _label_2
            (:`ApplyEasing`
              (`self.PointsFadeInPlayer` (`self.PointAdded`)))
            (:`OnComplete`
              (`KismetSystemLibrary.PrintText` "Fade In")
              (`FCTweenBPActionFloat.TweenFloat` 0.0
                (:`ApplyEasing`
                  (`self.PointsFadeOutPlayer`))
                (:`OnComplete`
                  (`KismetSystemLibrary.PrintText` "FadeOut")
                  (bind _gameplayhud (`self.GetUserHUDReference`))
                  (set `TextBlock.Text` (`KismetTextLibrary.Conv_IntToText` (`self.PlayerPoints`)) (`/Game/RTS/Blueprints/WidgetBP/HUD_WBP.PlayerDice_txt` _gameplayhud))))))
          (elif (`GameplayStatics.ObjectIsA` _array_element_2)
            (set `self.PointAdded` 2)
            (set `self.PlayerPoints` (+ (`self.PlayerPoints`) (`self.PointAdded`)))
            (goto _label_2)
            (elif (`GameplayStatics.ObjectIsA` _array_element_2 "/Game/RTS/Blueprints/CharactersBP/Enemy/EnemyLadron_BP.EnemyLadron_BP_C")
              (set `self.PointAdded` -2)
              (set `self.PlayerPoints` (+ (`self.PlayerPoints`) (`self.PointAdded`)))
              (goto _label_2)))))
      (elif (`GameplayStatics.ObjectIsA` _array_element "/Game/RTS/Blueprints/CharactersBP/Player/Constructor_BP.Constructor_BP_C")
        (for _array_element_3 (`self.EnemyCharacters`)
          (if (`GameplayStatics.ObjectIsA` _array_element_3 "/Game/RTS/Blueprints/CharactersBP/Enemy/EnemyRecolector_BP.EnemyRecolector_BP_C")
            (set `self.PointAdded` -2)
            (set `self.PlayerPoints` (+ (`self.PlayerPoints`) (`self.PointAdded`)))
            (goto _label_2)
            (elif (`GameplayStatics.ObjectIsA` _array_element_3)
              (set `self.PointAdded` 1)
              (set `self.PlayerPoints` (+ (`self.PlayerPoints`) (`self.PointAdded`)))
              (goto _label_2)
              (elif (`GameplayStatics.ObjectIsA` _array_element_3 "/Game/RTS/Blueprints/CharactersBP/Enemy/EnemyLadron_BP.EnemyLadron_BP_C")
                (set `self.PointAdded` 2)
                (set `self.PlayerPoints` (+ (`self.PlayerPoints`) (`self.PointAdded`)))
                (goto _label_2)))))
        (elif (`GameplayStatics.ObjectIsA` _array_element "/Game/RTS/Blueprints/CharactersBP/Player/Ladron_BP.Ladron_BP_C")
          (for _array_element_4 (`self.EnemyCharacters`)
            (if (`GameplayStatics.ObjectIsA` _array_element_4 "/Game/RTS/Blueprints/CharactersBP/Enemy/EnemyRecolector_BP.EnemyRecolector_BP_C")
              (set `self.PointAdded` 2)
              (set `self.PlayerPoints` (+ (`self.PlayerPoints`) (`self.PointAdded`)))
              (goto _label_2)
              (elif (`GameplayStatics.ObjectIsA` _array_element_4)
                (set `self.PointAdded` -2)
                (set `self.PlayerPoints` (+ (`self.PlayerPoints`) (`self.PointAdded`)))
                (goto _label_2)
                (elif (`GameplayStatics.ObjectIsA` _array_element_4 "/Game/RTS/Blueprints/CharactersBP/Enemy/EnemyLadron_BP.EnemyLadron_BP_C")
                  (set `self.PointAdded` 1)
                  (set `self.PlayerPoints` (+ (`self.PlayerPoints`) (`self.PointAdded`)))
                  (goto _label_2)))))))))
  ; EnemyPoints
  (for _array_element_5 (`self.EnemyCharacters`)
    (if (`GameplayStatics.ObjectIsA` _array_element_5 "/Game/RTS/Blueprints/CharactersBP/Enemy/EnemyRecolector_BP.EnemyRecolector_BP_C")
      (for _array_element_6 (`self.PlayerCharacters`)
        (if (`GameplayStatics.ObjectIsA` _array_element_6 "/Game/RTS/Blueprints/CharactersBP/Player/Recolector_BP.Recolector_BP_C")
          (set `self.PointAdded` 1)
          (set `self.EnemyPoints` (+ (`self.EnemyPoints`) (`self.PointAdded`)))
          (`FCTweenBPActionFloat.TweenFloat` 0.0 1.0 1.0 "Linear" :!label _label_3
            (:`ApplyEasing`
              (`self.PointsFadeInEnemy` (`self.PointAdded`)))
            (:`OnComplete`
              (`KismetSystemLibrary.PrintText` "Fade In")
              (`FCTweenBPActionFloat.TweenFloat` 0.0
                (:`ApplyEasing`
                  (`self.PointsFadeOutEnemy`))
                (:`OnComplete`
                  (`KismetSystemLibrary.PrintText` "FadeOut")
                  (bind _gameplayhud_2 (`self.GetUserHUDReference`))
                  (set `TextBlock.Text` (`KismetTextLibrary.Conv_IntToText` (`self.EnemyPoints`)) (`/Game/RTS/Blueprints/WidgetBP/HUD_WBP.EnemyDice_txt` _gameplayhud_2))))))
          (elif (`GameplayStatics.ObjectIsA` _array_element_6 "/Game/RTS/Blueprints/CharactersBP/Player/Constructor_BP.Constructor_BP_C")
            (set `self.PointAdded` 2)
            (set `self.EnemyPoints` (+ (`self.EnemyPoints`) (`self.PointAdded`)))
            (goto _label_3)
            (elif (`GameplayStatics.ObjectIsA` _array_element_6 "/Game/RTS/Blueprints/CharactersBP/Player/Ladron_BP.Ladron_BP_C")
              (set `self.PointAdded` -2)
              (set `self.EnemyPoints` (+ (`self.EnemyPoints`) (`self.PointAdded`)))
              (goto _label_3)))))
      (set `self.FightFinished` true)
      (elif (`GameplayStatics.ObjectIsA` _array_element_5)
        (for _array_element_7 (`self.PlayerCharacters`)
          (if (`GameplayStatics.ObjectIsA` _array_element_7 "/Game/RTS/Blueprints/CharactersBP/Player/Recolector_BP.Recolector_BP_C")
            (set `self.PointAdded` -2)
            (set `self.EnemyPoints` (+ (`self.EnemyPoints`) (`self.PointAdded`)))
            (goto _label_3)
            (elif (`GameplayStatics.ObjectIsA` _array_element_7 "/Game/RTS/Blueprints/CharactersBP/Player/Constructor_BP.Constructor_BP_C")
              (set `self.PointAdded` 1)
              (set `self.EnemyPoints` (+ (`self.EnemyPoints`) (`self.PointAdded`)))
              (goto _label_3)
              (elif (`GameplayStatics.ObjectIsA` _array_element_7 "/Game/RTS/Blueprints/CharactersBP/Player/Ladron_BP.Ladron_BP_C")
                (set `self.PointAdded` 2)
                (set `self.EnemyPoints` (+ (`self.EnemyPoints`) (`self.PointAdded`)))
                (goto _label_3)))))
        (elif (`GameplayStatics.ObjectIsA` _array_element_5 "/Game/RTS/Blueprints/CharactersBP/Enemy/EnemyLadron_BP.EnemyLadron_BP_C")
          (for _array_element_8 (`self.PlayerCharacters`)
            (if (`GameplayStatics.ObjectIsA` _array_element_8 "/Game/RTS/Blueprints/CharactersBP/Player/Recolector_BP.Recolector_BP_C")
              (set `self.PointAdded` 2)
              (set `self.EnemyPoints` (+ (`self.EnemyPoints`) (`self.PointAdded`)))
              (goto _label_3)
              (elif (`GameplayStatics.ObjectIsA` _array_element_8 "/Game/RTS/Blueprints/CharactersBP/Player/Constructor_BP.Constructor_BP_C")
                (set `self.PointAdded` -2)
                (set `self.EnemyPoints` (+ (`self.EnemyPoints`) (`self.PointAdded`)))
                (goto _label_3)
                (elif (`GameplayStatics.ObjectIsA` _array_element_8 "/Game/RTS/Blueprints/CharactersBP/Player/Ladron_BP.Ladron_BP_C")
                  (set `self.PointAdded` 1)
                  (set `self.EnemyPoints` (+ (`self.EnemyPoints`) (`self.PointAdded`)))
                  (goto _label_3))))))))))

(event `PointsFadeInPlayer`
  (params (Int :type Integer))
  ; FadeInPlayer Point
  (bind _gameplayhud (`self.GetUserHUDReference`))
  (bind _plusplayerpoints (`/Game/RTS/Blueprints/WidgetBP/HUD_WBP.PlusPlayerPoints` _gameplayhud))
  (set `TextBlock.Text` (`KismetTextLibrary.Conv_IntToText` Int) _plusplayerpoints)
  (`Widget.SetRenderOpacity` _plusplayerpoints 1.0)
  (bind (_rendertransform_translation _rendertransform_scale _rendertransform_shear _rendertransform_angle) (break `WidgetTransform` (`Widget.RenderTransform` _plusplayerpoints)))
  (bind (_x _y) (`KismetMathLibrary.BreakVector2D` _rendertransform_translation))
  (`Widget.SetRenderTransform` _plusplayerpoints (make `WidgetTransform` (`KismetMathLibrary.MakeVector2D` _x (+ _y -2.0)) _rendertransform_scale _rendertransform_shear _rendertransform_angle)))

(event `PointsFadeOutPlayer`
  ; FadeOut Player Points
  (bind _gameplayhud (`self.GetUserHUDReference`))
  (bind _plusplayerpoints (`/Game/RTS/Blueprints/WidgetBP/HUD_WBP.PlusPlayerPoints` _gameplayhud))
  (`Widget.SetRenderOpacity` _plusplayerpoints 0.0)
  (`TextBlock.SetOpacity` _plusplayerpoints 0.0)
  (set `Widget.RenderTransform` (make `WidgetTransform` (`/Game/RTS/Blueprints/WidgetBP/HUD_WBP.PlayerPlusPointPos` _gameplayhud)) _plusplayerpoints))

(event `PointsFadeInEnemy`
  (params (Int :type Integer))
  ; Fade In Enemy Points
  (bind _gameplayhud (`self.GetUserHUDReference`))
  (bind _plusenemypoints (`/Game/RTS/Blueprints/WidgetBP/HUD_WBP.PlusEnemyPoints` _gameplayhud))
  (set `TextBlock.Text` (`KismetTextLibrary.Conv_IntToText` Int) _plusenemypoints)
  (`Widget.SetRenderOpacity` _plusenemypoints 1.0)
  (bind (_rendertransform_translation _rendertransform_scale _rendertransform_shear _rendertransform_angle) (break `WidgetTransform` (`Widget.RenderTransform` _plusenemypoints)))
  (bind (_x _y) (`KismetMathLibrary.BreakVector2D` _rendertransform_translation))
  (`Widget.SetRenderTransform` _plusenemypoints (make `WidgetTransform` (`KismetMathLibrary.MakeVector2D` _x (+ _y -2.0)) _rendertransform_scale _rendertransform_shear _rendertransform_angle)))

(event `PointsFadeOutEnemy`
  ; Fade Out Enemy Point
  (bind _gameplayhud (`self.GetUserHUDReference`))
  (bind _plusenemypoints (`/Game/RTS/Blueprints/WidgetBP/HUD_WBP.PlusEnemyPoints` _gameplayhud))
  (`Widget.SetRenderOpacity` _plusenemypoints 0.0)
  (set `Widget.RenderTransform` (make `WidgetTransform` (`/Game/RTS/Blueprints/WidgetBP/HUD_WBP.EnemyPlusPointPos` _gameplayhud)) _plusenemypoints))

(fn `CharacterEnter`
  (params (Object :type "Object Object Reference"))
  (if (`GameplayStatics.ObjectIsA` Object "/Script/AquaRTS.CharacterRTS")
    (bind _ascharacter_rts (cast `CharacterRTS` Object))
    (set `CharacterRTS.isSafe` true _ascharacter_rts)
    (`KismetSystemLibrary.PrintText` "Safe")
    (`KismetSystemLibrary.PrintText` (`KismetTextLibrary.Conv_ObjectToText` _ascharacter_rts))
    (elif (`GameplayStatics.ObjectIsA` Object "/Script/AquaRTS.EnemyCharacterRTS")
      (bind _asenemy_character_rts (cast `EnemyCharacterRTS` Object))
      (set `EnemyCharacterRTS.isSafe` true _asenemy_character_rts)
      (`KismetSystemLibrary.PrintText` "Safe"))))

(fn `CharacterExit`
  (params (Object :type "Object Object Reference"))
  (if (`GameplayStatics.ObjectIsA` Object "/Script/AquaRTS.CharacterRTS")
    (bind _ascharacter_rts (cast `CharacterRTS` Object))
    (set `CharacterRTS.isSafe` false _ascharacter_rts)
    (`KismetSystemLibrary.PrintText` "Not Safe" true true (struct :`R` 1.0 :`B` 0.214979 :`A` 1.0))
    (elif (`GameplayStatics.ObjectIsA` Object "/Script/AquaRTS.EnemyCharacterRTS")
      (bind _asenemy_character_rts (cast `EnemyCharacterRTS` Object))
      (set `EnemyCharacterRTS.isSafe` false _asenemy_character_rts)
      (`KismetSystemLibrary.PrintText` "Not Safe" true true (struct :`R` 1.0 :`B` 0.214979 :`A` 1.0)))))

(fn `CheckForFight`
  (params (Actor :type "Actor Object Reference"))
  (returns (Check :type Boolean))
  (if (`|EnumEquality` (`self.TypeCaptured`) "NewEnumerator2")
    (if (`GameplayStatics.ObjectIsA` Actor "/Script/AquaRTS.CharacterRTS")
      (set `self.TypeCaptured` "NewEnumerator1")
      (`self.PlayerCaptured`)
      (set `self.FightCheck` false :!label _label)
      (return (`self.FightCheck`))
      (elif (`GameplayStatics.ObjectIsA` Actor "/Script/AquaRTS.EnemyCharacterRTS")
        (set `self.TypeCaptured` "NewEnumerator0")
        (`self.EnemyCaptured`)
        (goto _label)))
    (else
      (if (and (`|EnumEquality` (`self.TypeCaptured`) "NewEnumerator1") (`GameplayStatics.ObjectIsA` Actor "/Script/AquaRTS.CharacterRTS"))
        (set `self.FightCheck` false :!label _label_2)
        (elif (and (`|EnumEquality` (`self.TypeCaptured`) "NewEnumerator0") (`GameplayStatics.ObjectIsA` Actor "/Script/AquaRTS.EnemyCharacterRTS"))
          (goto _label_2)
          (else
            (set `self.FightCheck` true))))
      (return (`self.FightCheck`)))))

(fn `EnemyCaptured`
  (`WidgetComponent.SetTintColorAndOpacity` (`self.OverheadUI`) (struct :`R` 0.2 :`A` 0.8))
  (set `self.TypeCaptured` "NewEnumerator0"))

(fn `GetManagerReference`
  (returns (Manager :type "GameManager Object Reference"))
  (bind _asmy_game_manager (cast `/Game/RTS/Blueprints/MyGameManager` (`GameplayStatics.GetGameMode`)))
  (return _asmy_game_manager))

(fn `GetUserHUDReference`
  (returns (gameplayHud :type "/Game/RTS/Blueprints/WidgetBP/HUD_WBP Object Reference"))
  (bind _asmy_game_manager (cast `/Game/RTS/Blueprints/MyGameManager` (`GameplayStatics.GetGameMode`)))
  (return (`/Game/RTS/Blueprints/MyGameManager.HUDReference` _asmy_game_manager)))

(fn `PlayerCaptured`
  (`WidgetComponent.SetTintColorAndOpacity` (`self.OverheadUI`) (struct :`G` 0.2 :`B` 0.003428 :`A` 0.8))
  (set `self.TypeCaptured` "NewEnumerator1"))

(fn `ShowDice`
  (bind _manager (`self.GetManagerReference`))
  (bind _asmy_game_manager (cast `/Game/RTS/Blueprints/MyGameManager` _manager))
  (set `/Game/RTS/Blueprints/MyGameManager.EnemyDicePoints` 0 _asmy_game_manager)
  (set `/Game/RTS/Blueprints/MyGameManager.PlayerDicePoints` 0 _asmy_game_manager)
  (bind _gameplayhud (`self.GetUserHUDReference`))
  (`/Game/RTS/Blueprints/WidgetBP/HUD_WBP.ShowDicePanel` _gameplayhud)
  (set `TextBlock.Text` "0" (`/Game/RTS/Blueprints/WidgetBP/HUD_WBP.PlayerDice_txt` _gameplayhud))
  (set `TextBlock.Text` "0" (`/Game/RTS/Blueprints/WidgetBP/HUD_WBP.EnemyDice_txt` _gameplayhud))
  (bind _output_get (set `/Game/RTS/Blueprints/MyGameManager.EnemyDicePoints` (`KismetMathLibrary.Conv_Int64ToInt` (`KismetMathLibrary.RandomInteger64InRange` 1 6)) _asmy_game_manager))
  (set `self.EnemyPoints` _output_get)
  (bind _output_get_2 (set `/Game/RTS/Blueprints/MyGameManager.PlayerDicePoints` (`KismetMathLibrary.Conv_Int64ToInt` (`KismetMathLibrary.RandomInteger64InRange` 1 6)) _asmy_game_manager))
  (set `self.PlayerPoints` _output_get_2)
  (`KismetSystemLibrary.PrintText` (`KismetTextLibrary.Conv_IntToText` _output_get))
  (`KismetSystemLibrary.PrintText` (`KismetTextLibrary.Conv_IntToText` _output_get_2)))

(fn `UserConstructionScript`)

(fn `Winner`
  (if (> (`self.PlayerPoints`) (`self.EnemyPoints`))
    (for _array_element (`self.EnemyCharacters`)
      (`EnemyCharacterRTS.Die` _array_element))
    (`self.PlayerCaptured`)
    (`KismetArrayLibrary.Array_Clear` (`self.EnemyCharacters`))
    (`GameplayStatics.PlaySound2D` "/Game/RTS/Audio/FX/BattleWon.BattleWon" 1.0 1.0 0.0 null null)
    (else
      (for _array_element_2 (`self.PlayerCharacters`)
        (`CharacterRTS.Die` _array_element_2))
      (`self.EnemyCaptured`)
      (`KismetArrayLibrary.Array_Clear` (`self.PlayerCharacters`))
      (`GameplayStatics.PlaySound2D` "/Game/RTS/Audio/FX/BattleLose.BattleLose" 1.0 1.0 0.0 null null))))