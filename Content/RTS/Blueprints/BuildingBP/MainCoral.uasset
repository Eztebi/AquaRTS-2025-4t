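; MainCoral is an RTS building Blueprint for a coral structure, with a Fresnel material effect tied to clicking.
; On BeginPlay, its BPRuntimeMaterial component applies a runtime material to the Coral11 mesh and zeroes the FresnelMask parameter.
; The click handler runs a short linear float tween from the current FresnelMask, with no explicit end value, writing each step back to the material.
; The OnClicked binding sits inside that handler, not in BeginPlay.
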(event `OnClicked_Event` :!signature `self.OnClicked`
  (params (TouchedActor :type "Actor Object Reference") (ButtonPressed :type "Key Structure" :default "None"))
  (bind _runtimematerial (`/Game/RTS/Blueprints/BP_RuntimeMaterial.runtimeMaterial` (`self.BP_RuntimeMaterial`)))
  (add `self.OnClicked` (delegate `OnClicked_Event`))
  (bind _returnvalue (`MaterialInstanceDynamic.K2_GetScalarParameterValue` _runtimematerial (`self.fresnelMask`)))
  (bind (_asynctaskproxy _value) (`FCTweenBPActionFloat.TweenFloat` _returnvalue 1.0 0.3 "Linear")
    (:`ApplyEasing`
      (`MaterialInstanceDynamic.SetScalarParameterValue` _runtimematerial (`self.fresnelMask`) _value))))

(event `self.ReceiveBeginPlay`
  (bind _bp_runtimematerial (`self.BP_RuntimeMaterial`))
  (`/Game/RTS/Blueprints/BP_RuntimeMaterial.ApplyRuntimeMaterial` _bp_runtimematerial (`|MakeArray` (`self.coral_11`) null))
  (`MaterialInstanceDynamic.SetScalarParameterValue` (`/Game/RTS/Blueprints/BP_RuntimeMaterial.runtimeMaterial` _bp_runtimematerial) (`self.fresnelMask`) 0.0))

(fn `UserConstructionScript`)