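; RTS Guardian building that marks player and enemy RTS characters entering its sphere as IsSafe, ignoring Shark_BP.
; The exit handler is meant to clear that flag, but its casts are swapped between the two classes.
; Selection shows a marker, tweens a fresnel highlight and fills the HUD building panel.
; Deleting removes it from MyGameManager's list, then tweens its tint with camera shake and sound before destroying it.
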(event `self.Sphere1.OnComponentBeginOverlap`
  (params (OverlappedComponent :type "PrimitiveComponent Object Reference") (OtherActor :type "Actor Object Reference") (OtherComp :type "PrimitiveComponent Object Reference") (OtherBodyIndex :type Integer) (bFromSweep :type Boolean) (SweepResult :type "HitResult Structure (by ref)"))
  (if (not (`GameplayStatics.ObjectIsA` OtherActor "/Game/RTS/Blueprints/CharactersBP/Shark_BP.Shark_BP_C"))
    (`self.CharacterEnter` OtherActor)))

(event `ShakeCamera`
  (`PlayerCameraManager.StartCameraShake` :`self` (`PlayerController.PlayerCameraManager` (`GameplayStatics.GetPlayerController` 0)) :`ShakeClass` "/Game/RTS/Blueprints/CameraBP/BP_CameraShake.BP_CameraShake_C" :`Scale` 3.0)
  (`KismetSystemLibrary.PrintText` "Dead"))

(event `self.Sphere1.OnComponentEndOverlap`
  (params (OverlappedComponent :type "PrimitiveComponent Object Reference") (OtherActor :type "Actor Object Reference") (OtherComp :type "PrimitiveComponent Object Reference") (OtherBodyIndex :type Integer))
  (if (not (`GameplayStatics.ObjectIsA` OtherActor "/Game/RTS/Blueprints/CharactersBP/Shark_BP.Shark_BP_C"))
    (`self.CharacterExit` OtherActor)))

(event `Destroy`
  (bind _runtimematerial (`/Game/RTS/Blueprints/BP_RuntimeMaterial.runtimeMaterial` (`self.BP_RuntimeMaterial`)))
  (bind _returnvalue (`MaterialInstanceDynamic.K2_GetVectorParameterValue` _runtimematerial (`self.tintParameter`)))
  (bind (_asynctaskproxy _value) (`FCTweenBPActionVector.TweenVector` (`KismetMathLibrary.Conv_LinearColorToVector` _returnvalue) (`KismetMathLibrary.Conv_LinearColorToVector` (`KismetMathLibrary.Conv_ColorToLinearColor` (`self.TintColor`))))
    (:`then`
      (`self.ShakeCamera`)
      (`GameplayStatics.PlaySound2D` "/Game/RTS/Audio/FX/SC_BreakBuilding_Cue.SC_BreakBuilding_Cue" 1.0 1.0 0.0 null null))
    (:`ApplyEasing`
      (`MaterialInstanceDynamic.SetVectorParameterValue` _runtimematerial (`self.tintParameter`) (`KismetMathLibrary.Conv_VectorToLinearColor` _value)))
    (:`OnComplete`
      (`self.K2_DestroyActor`))))

(event `self.ReceiveBeginPlay`
  (bind _bp_runtimematerial (`self.BP_RuntimeMaterial`))
  ; Higlighter
  (`self.DeHighligthMarker`)
  (set `self.isSelected` false)
  (`/Game/RTS/Blueprints/BP_RuntimeMaterial.ApplyRuntimeMaterial` _bp_runtimematerial (`|MakeArray` (`self.Guardian`) :!type "MeshComponent Object Reference"))
  (`MaterialInstanceDynamic.SetScalarParameterValue` (`/Game/RTS/Blueprints/BP_RuntimeMaterial.runtimeMaterial` _bp_runtimematerial) (`self.fresnelMask`) 0.0))

(event `self.OnSelected`
  (bind _guardian (`self.Guardian`))
  (bind _runtimematerial (`/Game/RTS/Blueprints/BP_RuntimeMaterial.runtimeMaterial` (`self.BP_RuntimeMaterial`)))
  ; Higlighter
  ;; Appear
  (bind _output_get (set `self.isSelected` true))
  (bind _gameplayhud (`self.GetUserHUDReference`))
  (`/Game/RTS/Blueprints/WidgetBP/HUD_WBP.ShowBuildingSelection` _gameplayhud)
  (`self.ShowHudVariables`)
  (`self.HighligthMarker`)
  (bind _returnvalue (`MaterialInstanceDynamic.K2_GetScalarParameterValue` _runtimematerial (`self.fresnelMask`)))
  (bind (_asynctaskproxy _value) (`FCTweenBPActionFloat.TweenFloat` _returnvalue (`KismetMathLibrary.Conv_BoolToDouble` _output_get) 0.3 "Linear")
    (:`then`
      (`GameplayStatics.PlaySoundAtLocation` null (`SceneComponent.K2_GetComponentLocation` _guardian) (struct) 1.0 1.0 0.0 null null null null)
      (`KismetSystemLibrary.PrintText` (`KismetTextLibrary.Conv_StringToText` (`KismetStringLibrary.Concat_StrStr` "Selected" (`KismetSystemLibrary.GetDisplayName` _guardian)))))
    (:`ApplyEasing`
      (`MaterialInstanceDynamic.SetScalarParameterValue` _runtimematerial (`self.fresnelMask`) _value))))

(event `self.OnDeselected`
  (bind _runtimematerial (`/Game/RTS/Blueprints/BP_RuntimeMaterial.runtimeMaterial` (`self.BP_RuntimeMaterial`)))
  ; Higlighter
  ;; DisAppear
  (bind _output_get (set `self.isSelected` false))
  (bind _gameplayhud (`self.GetUserHUDReference`))
  (`/Game/RTS/Blueprints/WidgetBP/HUD_WBP.RemoveBuildingSelection` _gameplayhud)
  (`self.DeHighligthMarker`)
  (bind _returnvalue (`MaterialInstanceDynamic.K2_GetScalarParameterValue` _runtimematerial (`self.fresnelMask`)))
  (bind (_asynctaskproxy _value) (`FCTweenBPActionFloat.TweenFloat` _returnvalue (`KismetMathLibrary.Conv_BoolToDouble` _output_get) 0.3 "Linear")
    (:`then`
      (`KismetSystemLibrary.PrintText` "Deselected"))
    (:`ApplyEasing`
      (`MaterialInstanceDynamic.SetScalarParameterValue` _runtimematerial (`self.fresnelMask`) _value))))

(event `ShowHudVariables`
  ; Higlighter
  (if (`self.isSelected`)
    (bind _gameplayhud (`self.GetUserHUDReference`))
    (set `TextBlock.Text` (`KismetTextLibrary.Conv_StringToText` (`self.name`)) (`/Game/RTS/Blueprints/WidgetBP/HUD_WBP.BuildingName` _gameplayhud))
    (set `TextBlock.Text` (`KismetTextLibrary.Conv_StringToText` (`self.description`)) (`/Game/RTS/Blueprints/WidgetBP/HUD_WBP.BuildingDescription_txt` _gameplayhud))
    (bind _actionbuilding_btn (`/Game/RTS/Blueprints/WidgetBP/HUD_WBP.ActionBuilding_btn` _gameplayhud))
    (`Widget.SetVisibility` _actionbuilding_btn "SelfHitTestInvisible")
    (`Widget.SetRenderOpacity` _actionbuilding_btn 0.0)
    (clear `Button.OnClicked` _actionbuilding_btn)
    (add `Button.OnClicked` _actionbuilding_btn (delegate `OnAction`))
    (bind _deletebuilding_btn (`/Game/RTS/Blueprints/WidgetBP/HUD_WBP.DeleteBuilding_btn` _gameplayhud))
    (`Widget.SetVisibility` _deletebuilding_btn "Visible")
    (`Widget.SetRenderOpacity` _deletebuilding_btn 1.0)
    (add `Button.OnClicked` _deletebuilding_btn (delegate `DeleteFarm`))))

(event `OnAction`
  ; Higlighter
  (`KismetSystemLibrary.PrintText` "Nada"))

(event `DeleteFarm`
  ; Higlighter
  (bind _manager (`self.GetManagerReference`))
  (bind _asmy_game_manager (cast `/Game/RTS/Blueprints/MyGameManager` _manager))
  (bind _playerbuilding (`/Game/RTS/Blueprints/MyGameManager.PlayerBuilding` _asmy_game_manager))
  (for _array_element _playerbuilding
    (if (== _array_element self)
      (`ISelectionBuilding.OnDeselected`)
      (`KismetArrayLibrary.Array_RemoveItem` _playerbuilding _array_element)
      (`self.Destroy`))))

(fn `CharacterEnter`
  (params (Object :type "Object Object Reference"))
  (if (`GameplayStatics.ObjectIsA` Object "/Script/AquaRTS.CharacterRTS")
    (bind _ascharacter_rts (cast `CharacterRTS` Object))
    (set `CharacterRTS.isSafe` true _ascharacter_rts)
    (`KismetSystemLibrary.PrintText` "Safe")
    (`KismetSystemLibrary.PrintText` (`KismetTextLibrary.Conv_ObjectToText` _ascharacter_rts))
    (elif (`GameplayStatics.ObjectIsA` Object "/Script/AquaRTS.EnemyCharacterRTS")
      (bind _asenemy_character_rts (cast `EnemyCharacterRTS` Object))
      (set `EnemyCharacterRTS.isSafe` true _asenemy_character_rts)
      (`KismetSystemLibrary.PrintText` "Safe"))))

(fn `CharacterExit`
  (params (Object :type "Object Object Reference"))
  (if (`GameplayStatics.ObjectIsA` Object "/Script/AquaRTS.CharacterRTS")
    (bind _asenemy_character_rts (cast `EnemyCharacterRTS` Object))
    (set `EnemyCharacterRTS.isSafe` false _asenemy_character_rts)
    (elif (`GameplayStatics.ObjectIsA` Object "/Script/AquaRTS.EnemyCharacterRTS")
      (bind _ascharacter_rts (cast `CharacterRTS` Object))
      (set `CharacterRTS.isSafe` false _ascharacter_rts))))

(fn `DeHighligthMarker`
  (`SceneComponent.SetVisibility` (`self.SelectionMarker`) false false))

(fn `GetManagerReference`
  (returns (Manager :type "GameManager Object Reference"))
  (bind _asmy_game_manager (cast `/Game/RTS/Blueprints/MyGameManager` (`GameplayStatics.GetGameMode`)))
  (return _asmy_game_manager))

(fn `GetUserHUDReference`
  (returns (gameplayHud :type "/Game/RTS/Blueprints/WidgetBP/HUD_WBP Object Reference"))
  (bind _asmy_game_manager (cast `/Game/RTS/Blueprints/MyGameManager` (`GameplayStatics.GetGameMode`)))
  (return (`/Game/RTS/Blueprints/MyGameManager.HUDReference` _asmy_game_manager)))

(fn `HighligthMarker`
  (`SceneComponent.SetVisibility` (`self.SelectionMarker`) true false))

(fn `UserConstructionScript`)