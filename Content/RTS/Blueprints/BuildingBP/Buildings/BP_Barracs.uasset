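; Selectable RTS barracks building that spawns Recolector, Constructor and Ladron units at its own transform.
; Selection toggles the marker and HUD barracks panel, and tweens a FresnelMask highlight on a runtime material.
; On each selection it fills the panel text and binds the three spawn buttons and a delete button.
; Delete deselects the building, removes it from MyGameManager's PlayerBuilding list and destroys it.
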(event `self.ReceiveBeginPlay`
  (bind _bp_runtimematerial (`self.BP_RuntimeMaterial`))
  ; Higlighter
  (`self.DeHighligthMarker`)
  (set `self.isSelected` false)
  (`/Game/RTS/Blueprints/BP_RuntimeMaterial.ApplyRuntimeMaterial` _bp_runtimematerial (`|MakeArray` (`self.StaticMesh`) :!type "MeshComponent Object Reference"))
  (`MaterialInstanceDynamic.SetScalarParameterValue` (`/Game/RTS/Blueprints/BP_RuntimeMaterial.runtimeMaterial` _bp_runtimematerial) (`self.fresnelMask`) 0.0))

(event `self.OnSelected`
  (bind _staticmesh (`self.StaticMesh`))
  (bind _runtimematerial (`/Game/RTS/Blueprints/BP_RuntimeMaterial.runtimeMaterial` (`self.BP_RuntimeMaterial`)))
  ; Higlighter
  ;; Appear
  (bind _output_get (set `self.isSelected` true))
  (bind _gameplayhud (`self.GetUserHUDReference`))
  (`/Game/RTS/Blueprints/WidgetBP/HUD_WBP.ShowBarracsPanel` _gameplayhud)
  (`self.ShowHudVariables`)
  (`self.HighligthMarker`)
  (bind _returnvalue (`MaterialInstanceDynamic.K2_GetScalarParameterValue` _runtimematerial (`self.fresnelMask`)))
  (bind (_asynctaskproxy _value) (`FCTweenBPActionFloat.TweenFloat` _returnvalue (`KismetMathLibrary.Conv_BoolToDouble` _output_get) 0.3 "Linear")
    (:`then`
      (`GameplayStatics.PlaySoundAtLocation` "/Game/RTS/Audio/FX/SC_SelctedCharacter_Cue.SC_SelctedCharacter_Cue" (`SceneComponent.K2_GetComponentLocation` _staticmesh) (struct) 1.0 1.0 0.0 null null null null)
      (`KismetSystemLibrary.PrintText` (`KismetTextLibrary.Conv_StringToText` (`KismetStringLibrary.Concat_StrStr` "Selected" (`KismetSystemLibrary.GetDisplayName` _staticmesh)))))
    (:`ApplyEasing`
      (`MaterialInstanceDynamic.SetScalarParameterValue` _runtimematerial (`self.fresnelMask`) _value))))

(event `Action1`
  (`|SpawnActorFromClass` "/Game/RTS/Blueprints/CharactersBP/Player/Recolector_BP.Recolector_BP_C" (`KismetMathLibrary.MakeTransform` (`KismetMathLibrary.MakeVector` (.x (.location (`self.GetTransform`))) (.y (.location (`self.GetTransform`))) (.z (.location (`self.GetTransform`)))) (.rotation (`self.GetTransform`))) "AdjustIfPossibleButAlwaysSpawn" "MultiplyWithRoot" null null))

(event `Action2`
  (`|SpawnActorFromClass` "/Game/RTS/Blueprints/CharactersBP/Player/Constructor_BP.Constructor_BP_C" (`KismetMathLibrary.MakeTransform` (`KismetMathLibrary.MakeVector` (.x (.location (`self.GetTransform`))) (.y (.location (`self.GetTransform`))) (.z (.location (`self.GetTransform`)))) (.rotation (`self.GetTransform`))) "AdjustIfPossibleButAlwaysSpawn" "MultiplyWithRoot" null null))

(event `self.OnDeselected`
  (bind _runtimematerial (`/Game/RTS/Blueprints/BP_RuntimeMaterial.runtimeMaterial` (`self.BP_RuntimeMaterial`)))
  ; Higlighter
  ;; DisAppear
  (bind _output_get (set `self.isSelected` false))
  (bind _gameplayhud (`self.GetUserHUDReference`))
  (`/Game/RTS/Blueprints/WidgetBP/HUD_WBP.RemoveBarracsPanel` _gameplayhud)
  (`self.DeHighligthMarker`)
  (bind _returnvalue (`MaterialInstanceDynamic.K2_GetScalarParameterValue` _runtimematerial (`self.fresnelMask`)))
  (bind (_asynctaskproxy _value) (`FCTweenBPActionFloat.TweenFloat` _returnvalue (`KismetMathLibrary.Conv_BoolToDouble` _output_get) 0.3 "Linear")
    (:`then`
      (`KismetSystemLibrary.PrintText` "Deselected"))
    (:`ApplyEasing`
      (`MaterialInstanceDynamic.SetScalarParameterValue` _runtimematerial (`self.fresnelMask`) _value))))

(event `Action3`
  (`|SpawnActorFromClass` "/Game/RTS/Blueprints/CharactersBP/Player/Ladron_BP.Ladron_BP_C" (`KismetMathLibrary.MakeTransform` (`KismetMathLibrary.MakeVector` (.x (.location (`self.GetTransform`))) (.y (.location (`self.GetTransform`))) (.z (.location (`self.GetTransform`)))) (.rotation (`self.GetTransform`))) "AdjustIfPossibleButAlwaysSpawn" "MultiplyWithRoot" null null))

(event `ShowHudVariables`
  ; Higlighter
  (bind _gameplayhud (`self.GetUserHUDReference`))
  (set `TextBlock.Text` (`KismetTextLibrary.Conv_StringToText` (`self.name`)) (`/Game/RTS/Blueprints/WidgetBP/HUD_WBP.BarracsName` _gameplayhud))
  (set `TextBlock.Text` (`KismetTextLibrary.Conv_StringToText` (`self.description`)) (`/Game/RTS/Blueprints/WidgetBP/HUD_WBP.BarracDescription_txt` _gameplayhud))
  (add `Button.OnClicked` (`/Game/RTS/Blueprints/WidgetBP/HUD_WBP.ActionBarracs1_btn` _gameplayhud) (delegate `Action1_btn`))
  (set `TextBlock.Text` "Recolector" (`/Game/RTS/Blueprints/WidgetBP/HUD_WBP.ActionBarracs_Txt_1` _gameplayhud))
  (add `Button.OnClicked` (`/Game/RTS/Blueprints/WidgetBP/HUD_WBP.ActionBarracs2_btn` _gameplayhud) (delegate `Action2_btn`))
  (set `TextBlock.Text` "Constructor" (`/Game/RTS/Blueprints/WidgetBP/HUD_WBP.ActionBarracs_Txt_2` _gameplayhud))
  (add `Button.OnClicked` (`/Game/RTS/Blueprints/WidgetBP/HUD_WBP.ActionBarracs3_btn` _gameplayhud) (delegate `Action3_btn`))
  (set `TextBlock.Text` "Ladrond" (`/Game/RTS/Blueprints/WidgetBP/HUD_WBP.ActionBarracs_Txt_3` _gameplayhud))
  (add `Button.OnClicked` (`/Game/RTS/Blueprints/WidgetBP/HUD_WBP.DeleteBarracas_btn_1` _gameplayhud) (delegate `DeleteButton`)))

(event `Action1_btn`
  ; Higlighter
  (`self.Action1`))

(event `Action2_btn`
  ; Higlighter
  (`self.Action2`))

(event `Action3_btn`
  ; Higlighter
  (`self.Action3`))

(event `DeleteButton`
  ; Higlighter
  (bind _manager (`self.GetManagerReference`))
  (bind _asmy_game_manager (cast `/Game/RTS/Blueprints/MyGameManager` _manager))
  (bind _playerbuilding (`/Game/RTS/Blueprints/MyGameManager.PlayerBuilding` _asmy_game_manager))
  (for _array_element _playerbuilding
    (if (== _array_element self)
      (`ISelectionBuilding.OnDeselected`)
      (`KismetArrayLibrary.Array_RemoveItem` _playerbuilding _array_element)
      (`self.K2_DestroyActor`)
      (`KismetSystemLibrary.PrintText` "Destoryed"))))

(fn `DeHighligthMarker`
  (`SceneComponent.SetVisibility` (`self.SelectionMarker`) false false))

(fn `GetManagerReference`
  (returns (Manager :type "GameManager Object Reference"))
  (bind _asmy_game_manager (cast `/Game/RTS/Blueprints/MyGameManager` (`GameplayStatics.GetGameMode`)))
  (return _asmy_game_manager))

(fn `GetUserHUDReference`
  (returns (gameplayHud :type "/Game/RTS/Blueprints/WidgetBP/HUD_WBP Object Reference"))
  (bind _asmy_game_manager (cast `/Game/RTS/Blueprints/MyGameManager` (`GameplayStatics.GetGameMode`)))
  (return (`/Game/RTS/Blueprints/MyGameManager.HUDReference` _asmy_game_manager)))

(fn `HighligthMarker`
  (`SceneComponent.SetVisibility` (`self.SelectionMarker`) true false))

(fn `UserConstructionScript`)