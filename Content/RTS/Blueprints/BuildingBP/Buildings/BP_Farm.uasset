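; BP_Farm is an RTS farm building that can be selected, damaged and destroyed.
; Selection events toggle a marker, swap Constructor materials through tweens and show or remove the building selection on the HUD fetched from MyGameManager.
; Damage lowers Health and applies BPRuntimeMaterial's damage material through a looping yoyo tween.
; At zero Health it switches to a damaged material, shakes the player camera and destroys itself after a delay.
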(event `self.ReceiveBeginPlay`
  ; Higlighter
  (`self.DeHighligthMarker`)
  (set `self.isSelected` false)
  (`/Game/RTS/Blueprints/BP_RuntimeMaterial.ApplyRuntimeMaterial` (`self.BP_RuntimeMaterial`) (`|MakeArray` (`self.StaticMesh`) :!type "MeshComponent Object Reference")))

(event `self.OnSelected`
  (bind _staticmesh (`self.StaticMesh`))
  ; Higlighter
  ;; Appear
  (`self.HighligthMarker`)
  (set `self.isSelected` true)
  (`FCTweenBPActionFloat.TweenFloat` 0.0 1.0 0.3 "Linear"
    (:`then`
      (`GameplayStatics.PlaySoundAtLocation` null (`SceneComponent.K2_GetComponentLocation` _staticmesh) (struct) 1.0 1.0 0.0 null null null null)
      (`KismetSystemLibrary.PrintText` (`KismetTextLibrary.Conv_StringToText` (`KismetStringLibrary.Concat_StrStr` "Selected" (`KismetSystemLibrary.GetDisplayName` _staticmesh))))
      (bind _gameplayhud (`self.GetUserHUDReference`))
      (`/Game/RTS/Blueprints/WidgetBP/HUD_WBP.ShowBuildingSelection` _gameplayhud))
    (:`ApplyEasing`
      (`PrimitiveComponent.SetMaterial` (`self.StaticMesh`) 0 "/Game/RTS/Material/Character/MI_PBR_ConstructorSelected.MI_PBR_ConstructorSelected"))))

(event `self.RecieveDamage_BP`
  (`self.DamageChangeMaterial`)
  (bind _output_get (set `self.health` (- (`self.health`) 20)))
  (if (<= _output_get 0)
    (`PrimitiveComponent.SetMaterial` (`self.StaticMesh`) 0 "/Game/RTS/Material/Building/Building/Farm/MI_PBR_FarmDamage.MI_PBR_FarmDamage")
    (`self.ShakeCamera`)
    (`KismetSystemLibrary.Delay` 1.0)
    (`self.K2_DestroyActor`)
    (else
      (`KismetSystemLibrary.PrintText` (`KismetTextLibrary.Conv_IntToText` _output_get)))))

(event `self.OnDeselected`
  ; Higlighter
  ;; DisAppear
  (`self.DeHighligthMarker`)
  (set `self.isSelected` false)
  (`FCTweenBPActionFloat.TweenFloat` 0.0 1.0 0.3 "Linear"
    (:`then`
      (`KismetSystemLibrary.PrintText` "Deselected")
      (bind _gameplayhud (`self.GetUserHUDReference`))
      (`/Game/RTS/Blueprints/WidgetBP/HUD_WBP.RemoveBuildingSelection` _gameplayhud))
    (:`ApplyEasing`
      (`PrimitiveComponent.SetMaterial` (`self.StaticMesh`) 0 "/Game/RTS/Material/Character/MI_PBR_Constructor.MI_PBR_Constructor"))))

(event `ShakeCamera`
  (`PlayerCameraManager.StartCameraShake` :`self` (`PlayerController.PlayerCameraManager` (`GameplayStatics.GetPlayerController` 0)) :`ShakeClass` "/Game/RTS/Blueprints/CameraBP/BP_CameraShake.BP_CameraShake_C" :`Scale` 3.0)
  (`KismetSystemLibrary.PrintText` "Dead"))

(event `DamageChangeMaterial`
  (bind (_asynctaskproxy _value) (`FCTweenBPActionFloat.TweenFloat` (`ActorComponent.GetComponentTickInterval` (`self.BP_RuntimeMaterial`)) (`MeshComponent.GetOverlayMaterialMaxDrawDistance` (`self.StaticMesh`)) 1.0 "Linear" 0.0 0.0 0.3 3 0.0 true 0.3)
    (:`then`
      (`MeshComponent.SetOverlayMaterialMaxDrawDistance` (`self.StaticMesh`) _value))
    (:`ApplyEasing`
      (`/Game/RTS/Blueprints/BP_RuntimeMaterial.ApplyDamageMaterial` (`self.BP_RuntimeMaterial`) (`|MakeArray` (`self.StaticMesh`) :!type "MeshComponent Object Reference")))))

(fn `DeHighligthMarker`
  (`SceneComponent.SetVisibility` (`self.SelectionMarker`) false false))

(fn `GetUserHUDReference`
  (returns (gameplayHud :type "/Game/RTS/Blueprints/WidgetBP/HUD_WBP Object Reference"))
  (bind _asmy_game_manager (cast `/Game/RTS/Blueprints/MyGameManager` (`GameplayStatics.GetGameMode`)))
  (return (`/Game/RTS/Blueprints/MyGameManager.HUDReference` _asmy_game_manager)))

(fn `HighligthMarker`
  (`SceneComponent.SetVisibility` (`self.SelectionMarker`) true false))

(fn `UserConstructionScript`
  (set `self.health` 100))