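; Main Coral building for the RTS, a selectable structure that takes damage and can be destroyed.
; Selection toggles a marker, swaps the mesh material, plays a sound on select and shows or removes the building panel in HUD_WBP.
; Each hit cuts Health and tweens a tint on the runtime material from BPRuntimeMaterial.
; At zero Health it swaps to a damage material, shakes the camera and destroys itself after a short delay.
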(event `CustomEvent`
  (set `self.health` 100)
  (`/Game/RTS/Blueprints/BP_RuntimeMaterial.ApplyRuntimeMaterial` (`self.BP_RuntimeMaterial`) (`|MakeArray` (`self.SM_MainCoral`) :!type "MeshComponent Object Reference")))

(event `self.ReceiveBeginPlay`
  ; Higlighter
  (`self.DeHighligthMarker`)
  (set `self.isSelected` false)
  (`/Game/RTS/Blueprints/BP_RuntimeMaterial.ApplyRuntimeMaterial` (`self.BP_RuntimeMaterial`) (`|MakeArray` (`self.SM_MainCoral`) :!type "MeshComponent Object Reference"))
  (bind _foundwidgets (`WidgetBlueprintLibrary.GetAllWidgetsOfClass` "/Game/RTS/Blueprints/WidgetBP/HUD_WBP.HUD_WBP_C" false))
  (for _array_element _foundwidgets
    (bind _output_get (set `self.HUDReference` _array_element))
    (`KismetSystemLibrary.PrintText` (`KismetTextLibrary.Conv_ObjectToText` _output_get))))

(event `self.OnSelected`
  (bind _sm_maincoral (`self.SM_MainCoral`))
  ; Higlighter
  ;; Appear
  (`self.HighligthMarker`)
  (set `self.isSelected` true)
  (`FCTweenBPActionFloat.TweenFloat` 0.0 1.0 0.3 "Linear"
    (:`then`
      _)
    (:`OnComplete`
      _))
  (`PrimitiveComponent.SetMaterial` (`self.SM_MainCoral`) 0 "/Game/RTS/Material/Character/MI_PBR_ConstructorSelected.MI_PBR_ConstructorSelected")
  (`GameplayStatics.PlaySoundAtLocation` null (`SceneComponent.K2_GetComponentLocation` _sm_maincoral) (struct) 1.0 1.0 0.0 null null null null)
  (`KismetSystemLibrary.PrintText` (`KismetTextLibrary.Conv_StringToText` (`KismetStringLibrary.Concat_StrStr` "Selected" (`KismetSystemLibrary.GetDisplayName` _sm_maincoral))))
  (bind _ashud_wbp (cast `/Game/RTS/Blueprints/WidgetBP/HUD_WBP` (`self.HUDReference`)))
  (`/Game/RTS/Blueprints/WidgetBP/HUD_WBP.ShowBuildingSelection` _ashud_wbp))

(event `self.RecieveDamage_BP`
  (bind _output_get (set `self.health` (- (`self.health`) 20)))
  (if (<= _output_get 0)
    (`PrimitiveComponent.SetMaterial` (`self.SM_MainCoral`) 0 "/Game/RTS/Material/Building/Building/MainBuilding/MI_PBR_MainCoralDamage.MI_PBR_MainCoralDamage")
    (`self.ShakeCamera`)
    (`KismetSystemLibrary.Delay` 1.0)
    (`self.K2_DestroyActor`)
    (else
      (`KismetSystemLibrary.PrintText` (`KismetTextLibrary.Conv_IntToText` _output_get))
      (`self.DamageChangeMaterial`))))

(event `ShakeCamera`
  (`PlayerCameraManager.StartCameraShake` :`self` (`PlayerController.PlayerCameraManager` (`GameplayStatics.GetPlayerController` 0)) :`ShakeClass` "/Game/RTS/Blueprints/CameraBP/BP_CameraShake.BP_CameraShake_C" :`Scale` 3.0)
  (`KismetSystemLibrary.PrintText` "Dead"))

(event `self.OnDeselected`
  ; Higlighter
  ;; DisAppear
  (`self.DeHighligthMarker`)
  (set `self.isSelected` false)
  (`FCTweenBPActionFloat.TweenFloat` 0.0 1.0 0.3 "Linear"
    (:`ApplyEasing`
      (`PrimitiveComponent.SetMaterial` (`self.SM_MainCoral`) 0 "/Game/RTS/Material/Character/MI_PBR_Constructor.MI_PBR_Constructor"))
    (:`OnComplete`
      (`KismetSystemLibrary.PrintText` "Deselected")
      (bind _ashud_wbp (cast `/Game/RTS/Blueprints/WidgetBP/HUD_WBP` (`self.HUDReference`)))
      (`/Game/RTS/Blueprints/WidgetBP/HUD_WBP.RemoveBuildingSelection` _ashud_wbp))))

(event `DamageChangeMaterial`
  (bind _runtimematerial (`/Game/RTS/Blueprints/BP_RuntimeMaterial.runtimeMaterial` (`self.BP_RuntimeMaterial`)))
  (bind _returnvalue (`MaterialInstanceDynamic.K2_GetVectorParameterValue` _runtimematerial (`self.tintParameter`)))
  (bind (_asynctaskproxy _value) (`FCTweenBPActionVector.TweenVector` (`KismetMathLibrary.Conv_LinearColorToVector` _returnvalue) (`KismetMathLibrary.Conv_LinearColorToVector` (`KismetMathLibrary.Conv_ColorToLinearColor` (`self.TintColor`))))
    (:`ApplyEasing`
      (`MaterialInstanceDynamic.SetVectorParameterValue` _runtimematerial (`self.tintParameter`) (`KismetMathLibrary.Conv_VectorToLinearColor` _value)))))

(fn `DeHighligthMarker`
  (`SceneComponent.SetVisibility` (`self.SelectionMarker`) false false))

(fn `HighligthMarker`
  (`SceneComponent.SetVisibility` (`self.SelectionMarker`) true false))

(fn `UserConstructionScript`
  (set `self.health` 100))