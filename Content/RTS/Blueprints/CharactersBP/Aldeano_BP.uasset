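; Villager (Aldeano) unit Blueprint for the RTS that gives visual feedback when selected or deselected.
; BeginPlay hides the SelectionMarker, calls MoveComponentTo and applies a runtime material to the marker.
; OnSelected and OnDeselected set IsSelected, toggle marker visibility and start short linear float tweens.
; The tweens' Yoyo and Apply Easing callbacks swap the mesh between selected and default villager materials, with no interpolated value used.
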(event `self.ReceiveBeginPlay`
  ; Higlighter
  (`self.DeHighligthMarker`)
  (`KismetSystemLibrary.MoveComponentTo` null)
  (`/Game/RTS/Blueprints/BP_RuntimeMaterial.ApplyRuntimeMaterial` (`self.BP_RuntimeMaterial`) (`|MakeArray` (`self.Selection Marker`) :!type "MeshComponent Object Reference")))

(event `self.OnSelected`
  ; Higlighter
  ;; Appear
  (`self.HighligthMarker`)
  (bind _output_get (set `self.isSelected` true))
  (`FCTweenBPActionFloat.TweenFloat` 0.0 1.0 0.3 "Linear" 0.0 0.0 0.0 (`KismetMathLibrary.Conv_BoolToInt` _output_get) 0.0 _output_get
    (:`OnYoyo`
      (`PrimitiveComponent.SetMaterial` (`self.Mesh`) 0 "/Game/RTS/Material/Character/MI_PBR_AldeanoSelected.MI_PBR_AldeanoSelected"))))

(event `self.OnDeselected`
  ; Higlighter
  ;; DisAppear
  (`self.DeHighligthMarker`)
  (set `self.isSelected` false)
  (`FCTweenBPActionFloat.TweenFloat` 0.0 1.0 0.3 "Linear"
    (:`ApplyEasing`
      (`PrimitiveComponent.SetMaterial` (`self.Mesh`) 0 "/Game/RTS/Material/Character/MI_PBR_Aldeano.MI_PBR_Aldeano"))))

(fn `DeHighligthMarker`
  (`SceneComponent.SetVisibility` (`self.Selection Marker`) false false))

(fn `HighligthMarker`
  (`SceneComponent.SetVisibility` (`self.Selection Marker`) true false))

(fn `UserConstructionScript`)