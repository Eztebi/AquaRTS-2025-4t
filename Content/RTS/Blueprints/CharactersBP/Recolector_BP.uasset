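; Gatherer unit for the RTS that shuttles between an assigned resource and the main coral.
; ActionBP sets the target, and box overlaps drive the loop: pause at the resource, return to a lazily cached BP_MainCoral, then head back.
; MoveBP clears the target for plain move orders.
; Selection events toggle a marker mesh, use tweens to swap materials, and show or remove the HUD's character selection.
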(event `self.Move_BP`
  (params (location :type "Vector Structure"))
  ; Move To Position
  (bind _output_get (set `self.direction` location))
  (set `self.isRecolecting` false)
  (set `self.ResourceActor` null)
  (`|AIMoveTo` self _output_get null))

(event `self.Action_BP`
  (params (tempTarget :type "Actor Object Reference"))
  ; Action Recolect or Destroy
  (bind _output_get (set `self.ResourceActor` tempTarget))
  (`KismetSystemLibrary.PrintText` (`KismetTextLibrary.Conv_ObjectToText` _output_get))
  (set `self.direction` (`self.K2_GetActorLocation` _output_get))
  (`GameplayStatics.PlaySoundAtLocation` "/Game/RTS/Audio/FX/SC_ActionCharacter_Cue.SC_ActionCharacter_Cue" (`SceneComponent.K2_GetComponentLocation` (`self.CapsuleComponent`)) (struct) 1.0 1.0 0.0 null null null null)
  (`|AIMoveTo` self (0.0 0.0 0.0) (`self.ResourceActor`)))

(event `self.ReceiveBeginPlay`
  ; Higlighter
  (`self.DeHighligthMarker`)
  (set `self.direction` (0.0 0.0 0.0))
  (`/Game/RTS/Blueprints/BP_RuntimeMaterial.ApplyRuntimeMaterial` (`self.BP_RuntimeMaterial`) (`|MakeArray` (`self.Mesh`) :!type "MeshComponent Object Reference"))
  (bind _foundwidgets (`WidgetBlueprintLibrary.GetAllWidgetsOfClass` "/Game/RTS/Blueprints/WidgetBP/HUD_WBP.HUD_WBP_C"))
  (for _array_element _foundwidgets
    (set `self.HUDReference` _array_element)))

(event `self.Box.OnComponentBeginOverlap`
  (params (OverlappedComponent :type "PrimitiveComponent Object Reference") (OtherActor :type "Actor Object Reference") (OtherComp :type "PrimitiveComponent Object Reference") (OtherBodyIndex :type Integer) (bFromSweep :type Boolean) (SweepResult :type "HitResult Structure (by ref)"))
  (bind _resourceactor (`self.ResourceActor`))
  (bind _returnvalue (`KismetSystemLibrary.IsValid` (`self.ResourceActor`)))
  ; Collision
  (if (and (`GameplayStatics.ObjectIsA` OtherActor "/Script/AquaRTS.Resource") _returnvalue)
    (`KismetSystemLibrary.PrintText` "Recolecting")
    (set `self.isRecolecting` true)
    (`KismetSystemLibrary.Delay` 2.0)
    (`GameplayStatics.PlaySoundAtLocation` null (0.0 0.0 0.0) (struct) 1.0 1.0 0.0 null null null null)
    (`self.ReturnToMainCoral`)
    (`KismetSystemLibrary.PrintText` "Returning")
    (elif (and (`GameplayStatics.ObjectIsA` OtherActor "/Game/RTS/Blueprints/BuildingBP/Buildings/BP_MainCoral.BP_MainCoral_C") _returnvalue)
      (`self.Action` _resourceactor)
      (`|AIMoveTo` self (0.0 0.0 0.0) _resourceactor))))

(event `self.OnSelected`
  ; Higlighter
  ;; Appear
  (`self.HighligthMarker`)
  (bind _output_get (set `self.isSelected` true))
  (`FCTweenBPActionFloat.TweenFloat` 0.0 1.0 0.3 "Linear" 0.0 0.0 0.0 (`KismetMathLibrary.Conv_BoolToInt` _output_get) 0.0 _output_get
    (:`then`
      (`GameplayStatics.PlaySoundAtLocation` (`self.selectedSFX`) (`SceneComponent.K2_GetComponentLocation` (`self.CapsuleComponent`)) (struct) 1.0 1.0 0.0 null null null null)
      (bind _ashud_wbp (cast `/Game/RTS/Blueprints/WidgetBP/HUD_WBP` (`self.HUDReference`)))
      (`/Game/RTS/Blueprints/WidgetBP/HUD_WBP.ShowCharacterSelection` _ashud_wbp))
    (:`OnYoyo`
      (`PrimitiveComponent.SetMaterial` (`self.Mesh`) 0 "/Game/RTS/Material/Character/MI_PBR_ConstructorSelected.MI_PBR_ConstructorSelected"))))

(event `ReturnToMainCoral`
  (bind _maincoral (`self.mainCoral`))
  (if (`KismetSystemLibrary.IsValid` _maincoral)
    (set `self.direction` (`self.K2_GetActorLocation` _maincoral))
    (`KismetSystemLibrary.PrintText` "going tomaincoral" true true (struct :`R` 1.0 :`B` 0.752942 :`A` 1.0) :!label _label)
    (bind _maincoral_2 (`self.mainCoral`)
      (:`then`
        (`|AIMoveTo` self (0.0 0.0 0.0) _maincoral_2 20.0))
      (:`else`))
    (else
      (bind _outactors (`GameplayStatics.GetAllActorsOfClass` "/Game/RTS/Blueprints/BuildingBP/Buildings/BP_MainCoral.BP_MainCoral_C"))
      (for _array_element _outactors
        (bind _output_get (set `self.mainCoral` _array_element))
        (set `self.direction` (`self.K2_GetActorLocation` _output_get))
        (goto _label)))))

(event `self.OnDeselected`
  ; Higlighter
  ;; DisAppear
  (`self.DeHighligthMarker`)
  (set `self.isSelected` false)
  (`FCTweenBPActionFloat.TweenFloat` 0.0 1.0 0.3 "Linear"
    (:`then`
      (bind _ashud_wbp (cast `/Game/RTS/Blueprints/WidgetBP/HUD_WBP` (`self.HUDReference`)))
      (`/Game/RTS/Blueprints/WidgetBP/HUD_WBP.RemoveCharacterSelection` _ashud_wbp))
    (:`ApplyEasing`
      (`PrimitiveComponent.SetMaterial` (`self.Mesh`) 0 "/Game/RTS/Material/Character/MI_PBR_Constructor.MI_PBR_Constructor"))))

(fn `DeHighligthMarker`
  (`SceneComponent.SetVisibility` (`self.StaticMesh`) false false))

(fn `HighligthMarker`
  (`SceneComponent.SetVisibility` (`self.StaticMesh`) true false))

(fn `UserConstructionScript`)