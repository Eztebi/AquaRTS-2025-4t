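; Enemy collector unit Blueprint for the RTS, which implements only the visual death sequence.
; DieBP flags the ABP_Recolector anim instance as dead and zeroes walk speed, stopping early if that cast fails.
; It then linearly tweens the DitherMask parameter on the runtime material to zero for a dithered fade, destroying the actor on completion.
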(event `self.Die_BP`
  (bind _dithermask (`self.ditherMask`))
  (bind _runtimematerial (`/Game/RTS/Blueprints/BP_RuntimeMaterial.runtimeMaterial` (`self.BP_RuntimeMaterial`)))
  ; Die
  (bind _asabp_recolector (cast `/Game/RTS/Blueprints/AnimationBP/RecolectorAnimation/ABP_Recolector` (`SkeletalMeshComponent.GetAnimInstance` (`self.Mesh`))))
  (set `/Game/RTS/Blueprints/AnimationBP/RecolectorAnimation/ABP_Recolector.dead` true _asabp_recolector)
  (set `CharacterMovementComponent.MaxWalkSpeed` 0.0 (`self.CharacterMovement`))
  (bind _returnvalue (`MaterialInstanceDynamic.K2_GetScalarParameterValue` _runtimematerial _dithermask))
  (bind (_asynctaskproxy _value) (`FCTweenBPActionFloat.TweenFloat` _returnvalue 0.0 2.0 "Linear" 0.0 0.0 2.0)
    (:`then`
      (`KismetSystemLibrary.PrintText` "Destoryed"))
    (:`ApplyEasing`
      (`MaterialInstanceDynamic.SetScalarParameterValue` _runtimematerial _dithermask _value))
    (:`OnComplete`
      (`self.K2_DestroyActor`))))

(fn `UserConstructionScript`)