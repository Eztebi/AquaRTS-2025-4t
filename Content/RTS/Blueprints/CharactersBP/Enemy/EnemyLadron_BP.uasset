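; Enemy thief (Ladron) character Blueprint for the RTS game, whose only logic here is its death sequence.
; DieBP sets the Dead flag on the thief's animation Blueprint and zeroes walk speed.
; It then linearly tweens the DitherMask parameter of the runtime material to zero for a dithered fade-out, and destroys the actor when the tween completes.
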(event `self.Die_BP`
  (bind _dithermask (`self.ditherMask`))
  (bind _runtimematerial (`/Game/RTS/Blueprints/BP_RuntimeMaterial.runtimeMaterial` (`self.BP_RuntimeMaterial`)))
  ; Die
  (bind _asabp_ladron (cast `/Game/RTS/Blueprints/AnimationBP/LadronAnimation/ABP_Ladron` (`SkeletalMeshComponent.GetAnimInstance` (`self.Mesh`))))
  (set `/Game/RTS/Blueprints/AnimationBP/LadronAnimation/ABP_Ladron.dead` true _asabp_ladron)
  (set `CharacterMovementComponent.MaxWalkSpeed` 0.0 (`self.CharacterMovement`))
  (bind _returnvalue (`MaterialInstanceDynamic.K2_GetScalarParameterValue` _runtimematerial _dithermask))
  (bind (_asynctaskproxy _value) (`FCTweenBPActionFloat.TweenFloat` _returnvalue 0.0 2.0 "Linear" 0.0 0.0 2.0)
    (:`then`
      (`KismetSystemLibrary.PrintText` "Destoryed"))
    (:`ApplyEasing`
      (`MaterialInstanceDynamic.SetScalarParameterValue` _runtimematerial _dithermask _value))
    (:`OnComplete`
      (`self.K2_DestroyActor`))))

(fn `UserConstructionScript`)