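; Shark AI predator that hunts both player (CharacterRTS) and enemy (EnemyCharacterRTS) units.
; It wanders between random navmesh points around itself until an unsafe unit enters its Detection volume, then pursues it with AI MoveTo.
; Its Box overlap kills the chased unit, after which it resumes patrolling.
; It also drops the chase when the target leaves Detection or becomes IsSafe, which Tick checks continuously.
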(event `self.ReceiveBeginPlay`
  (`self.Patrol`))

(event `self.Box.OnComponentBeginOverlap`
  (params (OverlappedComponent :type "PrimitiveComponent Object Reference") (OtherActor :type "Actor Object Reference") (OtherComp :type "PrimitiveComponent Object Reference") (OtherBodyIndex :type Integer) (bFromSweep :type Boolean) (SweepResult :type "HitResult Structure (by ref)"))
  (bind _chasecharacter (`self.ChaseCharacter`))
  (if (`self.IsChasing`)
    (if (== (`self.ChaseCharacter`) OtherActor)
      (if (`GameplayStatics.ObjectIsA` _chasecharacter "/Script/AquaRTS.CharacterRTS")
        (bind _ascharacter_rts (cast `CharacterRTS` (`self.ChaseCharacter`)))
        (`CharacterRTS.Die` _ascharacter_rts)
        (`self.Patrol` :!label _label)
        (elif (`GameplayStatics.ObjectIsA` _chasecharacter "/Script/AquaRTS.EnemyCharacterRTS")
          (bind _asenemy_character_rts (cast `EnemyCharacterRTS` (`self.ChaseCharacter`)))
          (`EnemyCharacterRTS.Die` _asenemy_character_rts)
          (goto _label))))))

(event `self.Detection.OnComponentBeginOverlap`
  (params (OverlappedComponent :type "PrimitiveComponent Object Reference") (OtherActor :type "Actor Object Reference") (OtherComp :type "PrimitiveComponent Object Reference") (OtherBodyIndex :type Integer) (bFromSweep :type Boolean) (SweepResult :type "HitResult Structure (by ref)"))
  (if (`self.IsChasing`)
    _
    (elif (`GameplayStatics.ObjectIsA` OtherActor "/Script/AquaRTS.CharacterRTS")
      (bind _ascharacter_rts (cast `CharacterRTS` OtherActor))
      (`KismetSystemLibrary.PrintText` "Enter Player")
      (if (`CharacterRTS.isSafe` _ascharacter_rts)
        (`self.Patrol`)
        (else
          (set `self.ChaseCharacter` OtherActor)
          (`self.Chase`)))
      (elif (`GameplayStatics.ObjectIsA` OtherActor "/Script/AquaRTS.EnemyCharacterRTS")
        (bind _asenemy_character_rts (cast `EnemyCharacterRTS` OtherActor))
        (`KismetSystemLibrary.PrintText` "Enter Enemy")
        (if (`EnemyCharacterRTS.isSafe` _asenemy_character_rts)
          (`self.Patrol`)
          (else
            (set `self.ChaseCharacter` OtherActor)
            (`self.Chase`)))))))

(event `Chase`
  (bind _chasecharacter (`self.ChaseCharacter`))
  (set `self.IsChasing` true)
  (if (`KismetSystemLibrary.IsValid` (`self.ChaseCharacter`))
    (if (`GameplayStatics.ObjectIsA` _chasecharacter "/Script/AquaRTS.CharacterRTS")
      (bind _ascharacter_rts (cast `CharacterRTS` _chasecharacter))
      (if (`CharacterRTS.isSafe` _ascharacter_rts)
        (set `self.ChaseCharacter` null)
        (`self.Patrol` :!label _label_2)
        (else
          (`|AIMoveTo` self (0.0 0.0 0.0) _chasecharacter 1.0 :!label _label_3)))
      (elif (`GameplayStatics.ObjectIsA` _chasecharacter "/Script/AquaRTS.EnemyCharacterRTS")
        (bind _asenemy_character_rts (cast `EnemyCharacterRTS` _chasecharacter))
        (if (`EnemyCharacterRTS.isSafe` _asenemy_character_rts)
          (set `self.ChaseCharacter` null)
          (goto _label_2)
          (else
            (goto _label_3)))))))

(event `self.Detection.OnComponentEndOverlap`
  (params (OverlappedComponent :type "PrimitiveComponent Object Reference") (OtherActor :type "Actor Object Reference") (OtherComp :type "PrimitiveComponent Object Reference") (OtherBodyIndex :type Integer))
  (if (== OtherActor (`self.ChaseCharacter`))
    (set `self.ChaseCharacter` null)
    (`self.Patrol`)))

(event `Patrol`
  (set `self.IsChasing` false)
  (bind _randomlocation (`NavigationSystemV1.K2_GetRandomLocationInNavigableRadius` (`self.K2_GetActorLocation` self) 2000.0 null null))
  (`|AIMoveTo` self _randomlocation null
    (:`OnSuccess`
      _)
    (:`OnFail`
      _))
  (if (`KismetSystemLibrary.IsValid` (`self.ChaseCharacter`))
    (if (`self.IsChasing`)
      (`self.Chase`)
      (else
        (`self.Patrol` :!label _label_4)))
    (else
      (goto _label_4))))

(event `self.ReceiveTick`
  (params (DeltaSeconds :type "Float (single-precision)"))
  (bind _chasecharacter (`self.ChaseCharacter`))
  (if (`KismetSystemLibrary.IsValid` _chasecharacter)
    (if (`GameplayStatics.ObjectIsA` _chasecharacter "/Script/AquaRTS.CharacterRTS")
      (bind _ascharacter_rts (cast `CharacterRTS` (`self.ChaseCharacter`)))
      (if (`CharacterRTS.isSafe` _ascharacter_rts)
        (set `self.ChaseCharacter` null)
        (`self.Patrol`))
      (elif (`GameplayStatics.ObjectIsA` _chasecharacter "/Script/AquaRTS.EnemyCharacterRTS")
        (bind _asenemy_character_rts (cast `EnemyCharacterRTS` (`self.ChaseCharacter`)))
        (if (`EnemyCharacterRTS.isSafe` _asenemy_character_rts)
          (set `self.ChaseCharacter` null)
          (`self.Patrol`))))))

(fn `CharacterEnter`
  (params (Object :type "Object Object Reference") (Object2 :type "Object Object Reference") (Object3 :type "Object Object Reference") (Object4 :type "Object Object Reference"))
  (if (`GameplayStatics.ObjectIsA` Object4 "/Script/AquaRTS.CharacterRTS")
    (bind _asenemy_character_rts (cast `EnemyCharacterRTS` Object2))
    (set `EnemyCharacterRTS.isSafe` true _asenemy_character_rts)
    (elif (`GameplayStatics.ObjectIsA` Object "/Script/AquaRTS.EnemyCharacterRTS")
      (bind _ascharacter_rts (cast `CharacterRTS` Object3))
      (set `CharacterRTS.isSafe` true _ascharacter_rts))))

(fn `CharacterExit`
  (params (Object :type "Object Object Reference") (Object2 :type "Object Object Reference") (Object3 :type "Object Object Reference") (Object4 :type "Object Object Reference"))
  (if (`GameplayStatics.ObjectIsA` Object4 "/Script/AquaRTS.CharacterRTS")
    (cast `EnemyCharacterRTS` Object2)
    (elif (`GameplayStatics.ObjectIsA` Object "/Script/AquaRTS.EnemyCharacterRTS")
      (cast `CharacterRTS` Object3))))

(fn `UserConstructionScript`)