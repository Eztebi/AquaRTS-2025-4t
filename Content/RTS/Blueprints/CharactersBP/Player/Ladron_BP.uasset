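; Player-controlled thief unit (Ladron) for the RTS that shuttles between a target Recolector and the main coral to steal.
; Move and action commands drive AIMoveTo, while box overlaps, gated by a stealing flag, send it back to BP_MainCoral and re-issue the action there.
; Selection toggles a marker and tweened material swap; single selection also fills the HUD and binds its action and delete buttons.
; Death deselects it and removes it from MyGameManager's character list.
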(event `self.Move_BP`
  (params (location :type "Vector Structure"))
  ; Move To Position
  (bind _output_get (set `self.direction` location))
  (set `self.isStealing` false)
  (`|AIMoveTo` self _output_get null))

(event `self.ReceiveBeginPlay`
  ; Higlighter
  (`self.DeHighligthMarker`)
  (set `self.direction` (0.0 0.0 0.0))
  (`/Game/RTS/Blueprints/BP_RuntimeMaterial.ApplyRuntimeMaterial` (`self.BP_RuntimeMaterial`) (`|MakeArray` (`self.Mesh`) :!type "MeshComponent Object Reference")))

(event `Actionbtn`
  ; Action
  (`KismetSystemLibrary.PrintText` (`KismetTextLibrary.Conv_ObjectToText` (`self.Recolector`)))
  (`GameplayStatics.PlaySoundAtLocation` "/Game/RTS/Audio/FX/SC_ActionCharacter_Cue.SC_ActionCharacter_Cue" (`SceneComponent.K2_GetComponentLocation` (`self.CapsuleComponent`)) (struct) 1.0 1.0 0.0 null null null null)
  (`|AIMoveTo` self (0.0 0.0 0.0) (`self.Recolector`)
    (:`then`
      (set `self.isStealing` true))))

(event `self.Action_BP`
  (params (tempTarget :type "Actor Object Reference"))
  ; Action
  (bind _output_get (set `self.Recolector` tempTarget))
  (`KismetSystemLibrary.PrintText` (`KismetTextLibrary.Conv_ObjectToText` _output_get))
  (`GameplayStatics.PlaySoundAtLocation` "/Game/RTS/Audio/FX/SC_ActionCharacter_Cue.SC_ActionCharacter_Cue" (`SceneComponent.K2_GetComponentLocation` (`self.CapsuleComponent`)) (struct) 1.0 1.0 0.0 null null null null)
  (`|AIMoveTo` self (0.0 0.0 0.0) (`self.Recolector`)
    (:`then`
      (set `self.isStealing` true))))

(event `self.OnSelected`
  ; Higlighter
  ;; Appear
  (bind _output_get (set `self.isSelected` true))
  (bind _gameplayhud (`self.GetUserHUDReference`))
  (`/Game/RTS/Blueprints/WidgetBP/HUD_WBP.ShowCharacterSelection` _gameplayhud)
  (`self.ShowHudVariables`)
  (`self.HighligthMarker`)
  (`FCTweenBPActionFloat.TweenFloat` 0.0 1.0 0.3 "Linear" 0.0 0.0 0.0 (`KismetMathLibrary.Conv_BoolToInt` _output_get) 0.0 _output_get
    (:`then`
      (`GameplayStatics.PlaySoundAtLocation` (`self.selectedSFX`) (`SceneComponent.K2_GetComponentLocation` (`self.CapsuleComponent`)) (struct) 1.0 1.0 0.0 null null null null))
    (:`OnYoyo`
      (`PrimitiveComponent.SetMaterial` (`self.Mesh`) 0 "/Game/RTS/Material/Character/Playable/MI_PBR_ConstructorSelected.MI_PBR_ConstructorSelected"))))

(event `self.Box.OnComponentBeginOverlap`
  (params (OverlappedComponent :type "PrimitiveComponent Object Reference") (OtherActor :type "Actor Object Reference") (OtherComp :type "PrimitiveComponent Object Reference") (OtherBodyIndex :type Integer) (bFromSweep :type Boolean) (SweepResult :type "HitResult Structure (by ref)"))
  (bind _recolector (`self.Recolector`))
  (bind _maincoral (`self.mainCoral`))
  ; Action
  ;; Colision
  (if (`self.isStealing`)
    (if (== OtherActor _recolector)
      (`self.ReturnToMainCoral`)
      (else
        (bind _asbp_main_coral (cast `/Game/RTS/Blueprints/BuildingBP/Buildings/BP_MainCoral` _maincoral))
        (for _array_element (`PrimitiveComponent.GetOverlappingActors` (`/Game/RTS/Blueprints/BuildingBP/Buildings/BP_MainCoral.Box` _asbp_main_coral) "Ladron_BP_C")
          (if (and (== OtherActor _maincoral) (== _array_element self))
            (`self.Action` _recolector)))))))

(event `self.OnSelectedMultiple`
  ; Higlighter
  ;; Appear
  (bind _output_get (set `self.isSelected` true))
  (`self.HighligthMarker`)
  (`FCTweenBPActionFloat.TweenFloat` 0.0 1.0 0.3 "Linear" 0.0 0.0 0.0 (`KismetMathLibrary.Conv_BoolToInt` _output_get) 0.0 _output_get
    (:`then`
      (`GameplayStatics.PlaySoundAtLocation` (`self.selectedSFX`) (`SceneComponent.K2_GetComponentLocation` (`self.CapsuleComponent`)) (struct) 1.0 1.0 0.0 null null null null))
    (:`OnYoyo`
      (`PrimitiveComponent.SetMaterial` (`self.Mesh`) 0 "/Game/RTS/Material/Character/Playable/MI_PBR_ConstructorSelected.MI_PBR_ConstructorSelected"))))

(event `ReturnToMainCoral`
  (bind _maincoral (`self.mainCoral`))
  ; Action
  ;; ReturnToMainCoral
  (`GameplayStatics.PlaySound2D` "/Game/RTS/Audio/FX/SC_CharacterRecolect_Cue.SC_CharacterRecolect_Cue" 1.0 1.0 0.0 null null)
  (if (`KismetSystemLibrary.IsValid` _maincoral)
    (set `self.direction` (`self.K2_GetActorLocation` _maincoral))
    (`KismetSystemLibrary.PrintText` "going tomaincoral" true true (struct :`R` 1.0 :`B` 0.752942 :`A` 1.0) :!label _label)
    (bind _maincoral_2 (`self.mainCoral`)
      (:`then`
        (`|AIMoveTo` self (0.0 0.0 0.0) _maincoral_2 20.0))
      (:`else`))
    (else
      (bind _outactors (`GameplayStatics.GetAllActorsOfClass` "/Game/RTS/Blueprints/BuildingBP/Buildings/BP_MainCoral.BP_MainCoral_C"))
      (for _array_element _outactors
        (bind _output_get (set `self.mainCoral` _array_element))
        (set `self.direction` (`self.K2_GetActorLocation` _output_get))
        (goto _label)))))

(event `self.OnDeselected`
  ; Higlighter
  ;; DisAppear
  (set `self.isSelected` false)
  (bind _gameplayhud (`self.GetUserHUDReference`))
  (`/Game/RTS/Blueprints/WidgetBP/HUD_WBP.RemoveCharacterSelection` _gameplayhud)
  (`self.DeHighligthMarker`)
  (`FCTweenBPActionFloat.TweenFloat` 0.0 1.0 0.3 "Linear"
    (:`ApplyEasing`
      (`PrimitiveComponent.SetMaterial` (`self.Mesh`) 0 "/Game/RTS/Material/Character/Playable/MI_PBR_Constructor.MI_PBR_Constructor"))))

(event `self.Die_BP`
  ; Die
  (bind _manager (`self.GetManagerReference`))
  (bind _asmy_game_manager (cast `/Game/RTS/Blueprints/MyGameManager` _manager))
  (bind _playercharacters (`/Game/RTS/Blueprints/MyGameManager.PlayerCharacters` _asmy_game_manager))
  (for _array_element _playercharacters
    (if (== _array_element self)
      (message `ISelectionTroop.OnDeselected` _array_element)
      (`KismetArrayLibrary.Array_RemoveItem` _playercharacters _array_element)
      (`self.K2_DestroyActor`)
      (`KismetSystemLibrary.PrintText` "Destoryed"))))

(event `ShowHudVariables`
  ; Higlighter
  (if (`self.isSelected`)
    (bind _gameplayhud (`self.GetUserHUDReference`))
    (set `TextBlock.Text` (`KismetTextLibrary.Conv_StringToText` (`self.name`)) (`/Game/RTS/Blueprints/WidgetBP/HUD_WBP.CharacterName` _gameplayhud))
    (set `TextBlock.Text` (`KismetTextLibrary.Conv_StringToText` (`self.description`)) (`/Game/RTS/Blueprints/WidgetBP/HUD_WBP.DescriptionCharacter` _gameplayhud))
    (add `Button.OnClicked` (`/Game/RTS/Blueprints/WidgetBP/HUD_WBP.Action_btn` _gameplayhud) (delegate `OnActionButton`))
    (add `Button.OnClicked` (`/Game/RTS/Blueprints/WidgetBP/HUD_WBP.Delete_btn` _gameplayhud) (delegate `DeleteButton`))
    (set `TextBlock.Text` (`KismetTextLibrary.Conv_StringToText` (`self.actionDescription`)) (`/Game/RTS/Blueprints/WidgetBP/HUD_WBP.CharacterAction_txt` _gameplayhud))))

(event `OnActionButton`
  ; Higlighter
  (`self.Actionbtn`))

(event `DeleteButton`
  ; Higlighter
  (`self.Die`))

(fn `DeHighligthMarker`
  (`SceneComponent.SetVisibility` (`self.StaticMesh`) false false))

(fn `GetManagerReference`
  (returns (Manager :type "GameManager Object Reference"))
  (bind _asmy_game_manager (cast `/Game/RTS/Blueprints/MyGameManager` (`GameplayStatics.GetGameMode`)))
  (return _asmy_game_manager))

(fn `GetUserHUDReference`
  (returns (gameplayHud :type "/Game/RTS/Blueprints/WidgetBP/HUD_WBP Object Reference"))
  (bind _asmy_game_manager (cast `/Game/RTS/Blueprints/MyGameManager` (`GameplayStatics.GetGameMode`)))
  (return (`/Game/RTS/Blueprints/MyGameManager.HUDReference` _asmy_game_manager)))

(fn `HighligthMarker`
  (`SceneComponent.SetVisibility` (`self.StaticMesh`) true false))

(fn `UserConstructionScript`)