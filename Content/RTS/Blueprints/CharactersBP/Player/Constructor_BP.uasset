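; Player constructor unit for the RTS that moves by AI MoveTo and builds structures.
; Selection toggles a marker and material; single selection also fills the game manager's HUD builder panel and binds its action and delete buttons.
; Action buttons store a building choice, but Construir checks Building1–3 instead and only implements spawning a farm after moving and waiting.
; DieBP deselects the unit, removes it from the manager's player list and destroys it.
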(event `self.ReceiveBeginPlay`
  ; Higlighter
  (`self.DeHighligthMarker`)
  (set `self.direction` (0.0 0.0 0.0))
  (`/Game/RTS/Blueprints/BP_RuntimeMaterial.ApplyRuntimeMaterial` (`self.BP_RuntimeMaterial`) (`|MakeArray` (`self.Mesh`) :!type "MeshComponent Object Reference"))
  (`self.SetUserHUDReference`))

(event `self.Move_BP`
  (params (location :type "Vector Structure"))
  ; Move To Position
  (bind _output_get (set `self.direction` location))
  (`|AIMoveTo` self _output_get null))

(event `self.OnSelected`
  ; Higlighter
  ;; Appear
  (bind _output_get (set `self.isSelected` true))
  (bind _gameplayhud (`self.GetUserHUDReference`))
  (`/Game/RTS/Blueprints/WidgetBP/HUD_WBP.ShowBuilderSelection` _gameplayhud)
  (`self.ShowHudVariables`)
  (`self.HighligthMarker`)
  (`FCTweenBPActionFloat.TweenFloat` 0.0 1.0 0.3 "Linear" 0.0 0.0 0.0 (`KismetMathLibrary.Conv_BoolToInt` _output_get) 0.0 _output_get
    (:`then`
      (`GameplayStatics.PlaySoundAtLocation` (`self.selectedSFX`) (`SceneComponent.K2_GetComponentLocation` (`self.CapsuleComponent`)) (struct) 1.0 1.0 0.0 null null null null))
    (:`OnYoyo`
      (`PrimitiveComponent.SetMaterial` (`self.Mesh`) 0 "/Game/RTS/Material/Character/MI_PBR_ConstructorSelected.MI_PBR_ConstructorSelected"))))

(event `Action1`
  ; Action
  (set `self.BuildingSelected` (`self.Building 1`))
  (set `self.hasSelectedBuilding` true))

(event `self.OnSelectedMultiple`
  ; Higlighter
  ;; Appear
  (bind _output_get (set `self.isSelected` true))
  (bind _gameplayhud (`self.GetUserHUDReference`))
  (`/Game/RTS/Blueprints/WidgetBP/HUD_WBP.RemoveBuilderSelection` _gameplayhud)
  (`self.HighligthMarker`)
  (`FCTweenBPActionFloat.TweenFloat` 0.0 1.0 0.3 "Linear" 0.0 0.0 0.0 (`KismetMathLibrary.Conv_BoolToInt` _output_get) 0.0 _output_get
    (:`then`
      (`GameplayStatics.PlaySoundAtLocation` (`self.selectedSFX`) (`SceneComponent.K2_GetComponentLocation` (`self.CapsuleComponent`)) (struct) 1.0 1.0 0.0 null null null null))
    (:`OnYoyo`
      (`PrimitiveComponent.SetMaterial` (`self.Mesh`) 0 "/Game/RTS/Material/Character/MI_PBR_ConstructorSelected.MI_PBR_ConstructorSelected"))))

(event `Action2`
  ; Action
  (set `self.BuildingSelected` (`self.Building 2`))
  (set `self.hasSelectedBuilding` true))

(event `Action3`
  ; Action
  (set `self.BuildingSelected` (`self.Building 3`))
  (set `self.hasSelectedBuilding` true))

(event `Construir`
  (params (Direction :type "Vector Structure"))
  ; Action
  (bind _output_get (set `self.direction` Direction))
  (`|AIMoveTo` self _output_get null 5.0 true
    (:`OnSuccess`
      (`KismetSystemLibrary.Delay` 2.0)
      (if (== (`self.Building 1`) "Granja")
        (`|SpawnActorFromClass` "/Game/RTS/Blueprints/BuildingBP/Buildings/BP_Farm.BP_Farm_C" (`KismetMathLibrary.MakeTransform` (.location (`self.GetTransform`)) (.rotation (`self.GetTransform`))) "Undefined" "MultiplyWithRoot" null null)
        (set `self.hasSelectedBuilding` false)
        (elif (== (`self.Building 2`) "Barracas")
          _
          (elif (== (`self.Building 3`) "Defensa")
            _))))))

(event `self.OnDeselected`
  ; Higlighter
  ;; DisAppear
  (set `self.hasSelectedBuilding` false)
  (set `self.isSelected` false)
  (bind _gameplayhud (`self.GetUserHUDReference`))
  (`/Game/RTS/Blueprints/WidgetBP/HUD_WBP.RemoveBuilderSelection` _gameplayhud)
  (`self.DeHighligthMarker`)
  (`FCTweenBPActionFloat.TweenFloat` 0.0 1.0 0.3 "Linear"
    (:`ApplyEasing`
      (`PrimitiveComponent.SetMaterial` (`self.Mesh`) 0 "/Game/RTS/Material/Character/MI_PBR_Constructor.MI_PBR_Constructor"))))

(event `self.Die_BP`
  ; Die
  (bind _manager (`self.GetManagerReference`))
  (bind _asmy_game_manager (cast `/Game/RTS/Blueprints/MyGameManager` _manager))
  (bind _playercharacters (`/Game/RTS/Blueprints/MyGameManager.PlayerCharacters` _asmy_game_manager))
  (for _array_element _playercharacters
    (if (== _array_element self)
      (message `ISelectionTroop.OnDeselected` _array_element)
      (`KismetArrayLibrary.Array_RemoveItem` _playercharacters _array_element)
      (`self.K2_DestroyActor`)
      (`KismetSystemLibrary.PrintText` "Destoryed"))))

(event `ShowHudVariables`
  ; Higlighter
  (bind _gameplayhud (`self.GetUserHUDReference`))
  (set `TextBlock.Text` (`KismetTextLibrary.Conv_StringToText` (`self.name`)) (`/Game/RTS/Blueprints/WidgetBP/HUD_WBP.BuilderName` _gameplayhud))
  (set `TextBlock.Text` (`KismetTextLibrary.Conv_StringToText` (`self.description`)) (`/Game/RTS/Blueprints/WidgetBP/HUD_WBP.BuilderDescription_txt` _gameplayhud))
  (add `Button.OnClicked` (`/Game/RTS/Blueprints/WidgetBP/HUD_WBP.BuilderAction1_btn` _gameplayhud) (delegate `Action1_btn`))
  (set `TextBlock.Text` (`KismetTextLibrary.Conv_StringToText` (`self.Action1Name`)) (`/Game/RTS/Blueprints/WidgetBP/HUD_WBP.BuilderAction1_txt` _gameplayhud))
  (add `Button.OnClicked` (`/Game/RTS/Blueprints/WidgetBP/HUD_WBP.BuilderAction2_btn` _gameplayhud) (delegate `Action2_btn`))
  (set `TextBlock.Text` (`KismetTextLibrary.Conv_StringToText` (`self.Action2Name`)) (`/Game/RTS/Blueprints/WidgetBP/HUD_WBP.BuilderAction2_txt` _gameplayhud))
  (add `Button.OnClicked` (`/Game/RTS/Blueprints/WidgetBP/HUD_WBP.BuilderAction3_btn` _gameplayhud) (delegate `Action3_btn`))
  (set `TextBlock.Text` (`KismetTextLibrary.Conv_StringToText` (`self.Action3Name`)) (`/Game/RTS/Blueprints/WidgetBP/HUD_WBP.BuilderAction3_txt` _gameplayhud))
  (add `Button.OnClicked` (`/Game/RTS/Blueprints/WidgetBP/HUD_WBP.DeleteBuilder_btn` _gameplayhud) (delegate `DeleteButton`)))

(event `Action1_btn`
  ; Higlighter
  (`self.Action1`))

(event `Action2_btn`
  ; Higlighter
  (`self.Action2`))

(event `Action3_btn`
  ; Higlighter
  (`self.Action3`))

(event `DeleteButton`
  ; Higlighter
  (`self.Die`))

(fn `DeHighligthMarker`
  (`SceneComponent.SetVisibility` (`self.StaticMesh`) false false))

(fn `GetManagerReference`
  (returns (Manager :type "GameManager Object Reference"))
  (bind _asmy_game_manager (cast `/Game/RTS/Blueprints/MyGameManager` (`GameplayStatics.GetGameMode`)))
  (return _asmy_game_manager))

(fn `GetUserHUDReference`
  (returns (gameplayHud :type "/Game/RTS/Blueprints/WidgetBP/HUD_WBP Object Reference"))
  (bind _asmy_game_manager (cast `/Game/RTS/Blueprints/MyGameManager` (`GameplayStatics.GetGameMode`)))
  (return (`/Game/RTS/Blueprints/MyGameManager.HUDReference` _asmy_game_manager)))

(fn `HighligthMarker`
  (`SceneComponent.SetVisibility` (`self.StaticMesh`) true false))

(fn `SetUserHUDReference`
  (bind _foundwidgets (`WidgetBlueprintLibrary.GetAllWidgetsOfClass` "/Script/UMG.UserWidget"))
  (for _array_element _foundwidgets
    (if (`GameplayStatics.ObjectIsA` _array_element "/Game/RTS/Blueprints/WidgetBP/HUD_WBP.HUD_WBP_C")
      (set `self.HUDReference` _array_element))))

(fn `UserConstructionScript`)